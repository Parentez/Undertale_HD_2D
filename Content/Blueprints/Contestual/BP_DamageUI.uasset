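; BP_DamageUI is a contextual damage display actor with five hit zones, each mapped to a float value, likely a damage multiplier, on BeginPlay.
; Show and hide events use timelines to grow or collapse its Z scale, toggling actor visibility around the animation.
; Each timeline fires a finished dispatcher for other logic to react to.
; The file itself never applies the zone values; only a disconnected debug print reads them.
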(event Custom|Show%20Damage%20dealer
  (Rendering|SetActorHiddenInGame false)
  (bind _increase_scale (Timeline|Increase%20self PlayFromStart)
    (:Update
      (Transformation|SetActorRelativeScale3D (Math|Vector|Lerp(Vector) "1.600000,1.000000,0.000000" "1.600000,1.000000,1.300000" _increase_scale)))
    (:Finished
      (Default|CallOnIncreaseFinished))))

(event Custom|Hide%20Damage%20dealer
  (bind _decrease_scale (Timeline|Timeline PlayFromStart)
    (:Update
      (Transformation|SetActorRelativeScale3D (Math|Vector|Lerp(Vector) "1.600000,1.000000,1.300000" "1.600000,1.000000,0.000000" _decrease_scale)))
    (:Finished
      (Rendering|SetActorHiddenInGame true)
      (Default|CallOnDecreaseFinished))))

(event EventBeginPlay
  (bind _hitzones (Variables|Default|GetHitZones))
  (Utilities|Map|Add _hitzones (Variables|Default|GetHitzone1) 0.5)
  (Utilities|Map|Add _hitzones (Variables|Default|GetHitzone2) 1.5)
  (Utilities|Map|Add _hitzones (Variables|Default|GetHitzone3) 1.5)
  (Utilities|Map|Add _hitzones (Variables|Default|GetHitzone4) 0.5)
  (Utilities|Map|Add _hitzones (Variables|Default|GetHitzone5) 2.0))

(fn ConstructionScript)