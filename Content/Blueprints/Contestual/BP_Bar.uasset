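; BP_Bar is a sprite-based actor that slides along a fixed horizontal path, apparently a bar in an enemy encounter.
; On BeginPlay it enables player input, caches the tagged BP_Enemy and runs a timeline that lerps its Y position at constant X.
; When the timeline finishes, it asks the enemy to remove it from its array.
; StopMovement halts the timeline, clears the sprite and switches the flipbook to a first-attack animation.
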(event Custom|Stop%20Movement
  (bind _self self)
  (bind _returnvalue (Transformation|GetActorLocation _self))
  (Rendering|Components|Sprite|SetSprite (Variables|Default|GetRenderComponent) 0)
  (Sprite|SetFlipbook (Variables|Default|GetPaperFlipbook) "/Game/Sprite/UI/SP_first_attack.SP_first_attack")
  (bind _bar_movement (Timeline|Timeline Stop)
    (:Update
      (Transformation|SetActorLocation (Math|Vector|Lerp(Vector) (Math|Vector|MakeVector -946.700012 6.4e+03 (.z _returnvalue)) (Math|Vector|MakeVector -946.700012 4.2e+03 (.z _returnvalue)) _bar_movement) false false))
    (:Finished
      (Default|RemoveBarfromArray (Variables|Default|GetBP%20enemy) self))))

(event EventBeginPlay
  (bind _self self)
  (bind _returnvalue (Transformation|GetActorLocation _self))
  (bind _outactors (Actor|GetAllActorsOfClasswithTag "/Game/Blueprints/Battles/Enemies/BP_Enemy.BP_Enemy_C" "BP_Enemy"))
  (Variables|Default|SetBP%20enemy (Utilities|Array|Get(acopy) _outactors))
  (Input|EnableInput (Game|GetPlayerController 0))
  (bind _bar_movement (Timeline|Timeline PlayFromStart)
    (:Update
      (Transformation|SetActorLocation (Math|Vector|Lerp(Vector) (Math|Vector|MakeVector -946.700012 6.4e+03 (.z _returnvalue)) (Math|Vector|MakeVector -946.700012 4.2e+03 (.z _returnvalue)) _bar_movement) false false))
    (:Finished
      (Default|RemoveBarfromArray (Variables|Default|GetBP%20enemy) self))))

(fn ConstructionScript)