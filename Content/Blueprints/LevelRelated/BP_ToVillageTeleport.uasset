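; Trigger actor that moves the player to the village when their character overlaps it.
; On overlap it sets the player's village and area flags and plays a fade widget created at BeginPlay.
; After a short delay it disables movement and relocates the player to VillageSpawnPoint, then switches movement to NavWalking after another delay.
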(event Collision|EventActorBeginOverlap
  (params (OtherActor :type Actor%20Object%20Reference))
  (bind _player (Variables|Default|GetPlayer))
  (bind _fadewidget (Variables|Default|GetFadeWidget))
  (bind _player_2 (Variables|Default|GetPlayer))
  (if (== OtherActor (Game|GetPlayerCharacter 0))
    (Variables|/Script/Undertale_HD_2D.MyPlayerCharacter|SetbInVillage _player true)
    (Variables|/Script/Undertale_HD_2D.MyPlayerCharacter|SetbInArea1 _player false)
    (UserInterface|Viewport|AddtoViewport _fadewidget 0)
    (Variables|/Game/UI/Combat/WB_Fade.WB_Fade_C|SetDuration _fadewidget 1.0)
    (Default|Fade _fadewidget)
    (Utilities|FlowControl|Delay 0.5)
    (Pawn|Components|CharacterMovement|DisableMovement (Variables|/Script/Engine.Character|GetCharacterMovement _player_2))
    (Transformation|SetActorLocation _player_2 (Transformation|GetActorLocation (Variables|Default|GetVillageSpawnPoint)) false false)
    (Utilities|FlowControl|Delay 1.0)
    (Pawn|Components|CharacterMovement|SetMovementMode (Variables|/Script/Engine.Character|GetCharacterMovement (Variables|Default|GetPlayer)) "MOVE_NavWalking" 0)))

(event EventBeginPlay
  (bind _outactors (Actor|GetAllActorsOfClasswithTag "/Game/Blueprints/MainCharacter/NormalPlayer/BP_PlayerCharacter.BP_PlayerCharacter_C" "Player Character"))
  (Variables|Default|SetPlayer (Utilities|Array|Get(acopy) _outactors))
  (bind _returnvalue (UserInterface|CreateWidget "/Game/UI/Combat/WB_Fade.WB_Fade_C"))
  (Variables|Default|SetFadeWidget _returnvalue))

(fn ConstructionScript)