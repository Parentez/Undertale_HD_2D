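; BP_PlayerHeart is the player-controlled heart in battle, moved with Enhanced Input and carrying its own HP.
; On BeginPlay it finds the tagged BP_BattleManager, pushes health to its UI and adds the default mapping context.
; TakeDamage updates that UI and turns the HP text red at low health.
; At zero HP, DeathCall destroys the heart, shows the death screen widget and switches to UI-only input.
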(event Input|EnhancedActionEvents|EnhancedInputActionIA_MoveHeart
  (params (ActionValue :type Vector%202D%20Structure) (ElapsedSeconds :type Float%20%28double-precision%29) (TriggeredSeconds :type Float%20%28double-precision%29) (InputAction :type Input%20Action%20Object%20Reference :default "/Game/Inputs/IA_MoveHeart.IA_MoveHeart"))
  (bind _returnvalue (Pawn|GetControlRotation :!class /Script/Engine.Pawn))
  ;[0.3086 0.6542 0.9115] Movement SetUp
  (Pawn|Input|AddMovementInput (Math|Vector|GetRightVector (Math|Rotator|MakeRotator (.roll _returnvalue) 0.0 (.yaw _returnvalue))) (.x ActionValue) false)
  (Pawn|Input|AddMovementInput (Math|Vector|GetForwardVector (Math|Rotator|MakeRotator 0.0 0.0 (.yaw (Pawn|GetControlRotation :!class /Script/Engine.Pawn)))) (.y ActionValue) false))

(event EventBeginPlay
  ;[1 1 1] Set Input Context
  (bind _outactors (Actor|GetAllActorsOfClasswithTag "/Game/Blueprints/Battles/BP_BattleManager.BP_BattleManager_C" "BP_BattleManager"))
  (bind _output_get (Variables|Default|SetBattleManager (Utilities|Array|Get(acopy) _outactors)))
  (Default|UpdateHealthUi _output_get (Variables|Default|GetHP) (Variables|Default|GetMax%20HP))
  (bind _asplayer_controller (Utilities|Casting|CastToPlayerController (Pawn|GetController)))
  (Utilities|IsValid (PlayerController|LocalPlayerSubsystems|GetEnhancedInputLocalPlayerSubsystem _asplayer_controller)
    (:Is%20Valid
      (Input|AddMappingContext (PlayerController|LocalPlayerSubsystems|GetEnhancedInputLocalPlayerSubsystem _asplayer_controller) "/Game/Inputs/IMC_Default.IMC_Default" 0 "(bIgnoreAllPressedKeysUntilRelease=True,bForceImmediately=False,bNotifyUserSettings=False)"))))

(fn ConstructionScript)

(fn TakeDamage
  (params (Damage :type Integer))
  (bind _output_get (Variables|Default|SetHP (- (Variables|Default|GetHP) Damage)))
  (Default|UpdateHealthUi (Variables|Default|GetBattleManager) _output_get (Variables|Default|GetMax%20HP))
  (if (<= (Variables|Default|GetHP) 35)
    (Appearance|SetColorandOpacity (Variables|/Game/UI/Combat/WB_PlayerHealth.WB_PlayerHealth_C|GetCurrentHP (Variables|/Game/Blueprints/Battles/BP_BattleManager.BP_BattleManager_C|GetHealth%20Wid (Variables|Default|GetBattleManager))) (Utilities|Struct|MakeSlateColor "(R=1.000000,G=0.009271,B=0.000000,A=1.000000)" "UseColor_Specified") :!class /Script/UMG.TextBlock)
    (if (<= (Variables|Default|GetHP) 0)
      (CallFunction|DeathCall))))

(fn DeathCall
  (Actor|DestroyActor)
  (bind _returnvalue (UserInterface|CreateWidget "/Game/UI/Combat/WB_DeathScene.WB_DeathScene_C"))
  (bind _output_get (Variables|Default|SetDeathWidget _returnvalue))
  (UserInterface|Viewport|AddtoViewport _output_get 0)
  (Input|SetInputModeUIOnly (Game|GetPlayerController 0) 0 "DoNotLock" false))