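; Player character Blueprint that handles NPC interaction and dialogue, plus a camera zoom transition.
; An overlap radius finds interactable NPCs through BPI_npcInteractable, shows their key prompt and stores references.
; Input starts the interaction, freezing movement and optionally repositioning the player, or skips dialogue; ClearReferences restores movement and the camera view.
; ZoomTransition animates FOV with a timeline while switching depth-of-field focal distance.
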(event OnComponentBeginOverlap(InteractableRadius)
  (params (OverlappedComponent :type Primitive%20Component%20Object%20Reference) (OtherActor :type Actor%20Object%20Reference) (OtherComp :type Primitive%20Component%20Object%20Reference) (OtherBodyIndex :type Integer) (bFromSweep :type Boolean) (SweepResult :type Hit%20Result%20Structure%20%28by%20ref%29))
  (if (!= OtherActor self)
    (if (Utilities|DoesObjectImplementInterface OtherActor "/Game/Blueprints/NPC/BPI_npcInteractable.BPI_npcInteractable_C")
      (bind _asbp_npc (Utilities|Casting|CastToBP_NPC OtherActor))
      (bind _output_get (Variables|Default|SetNPC _asbp_npc))
      (Default|EKeyVisible _output_get)
      (bind _output_get_2 (Variables|Default|SetInteractable%20Npc _output_get))
      (Class|BPINpcInteractable|SetInteractableState(Message) _output_get_2 true))))

(event OnComponentEndOverlap(InteractableRadius)
  (params (OverlappedComponent :type Primitive%20Component%20Object%20Reference) (OtherActor :type Actor%20Object%20Reference) (OtherComp :type Primitive%20Component%20Object%20Reference) (OtherBodyIndex :type Integer))
  (bind _npc (Variables|Default|GetNPC))
  (if (and (!= OtherActor self) (== OtherActor (Variables|Default|GetInteractable%20Npc)))
    (Class|BPINpcInteractable|SetInteractableState(Message) (Variables|Default|GetInteractable%20Npc) false)
    (Utilities|IsValid _npc
      (:Is%20Valid
        (Default|HideEKey _npc)))))

(event Input|EnhancedActionEvents|EnhancedInputActionIA_InteractWNpc
  (params (ActionValue :type Boolean) (ElapsedSeconds :type Float%20%28double-precision%29) (TriggeredSeconds :type Float%20%28double-precision%29) (InputAction :type Input%20Action%20Object%20Reference :default "/Game/Inputs/IA_InteractWNpc.IA_InteractWNpc"))
  (bind _self self)
  (bind _npc (Variables|Default|GetNPC))
  (:Started
    (Utilities|IsValid (Variables|Default|GetInteractable%20Npc)
      (:Is%20Valid
        (if (not (Variables|/Game/Blueprints/NPC/BP_NPC.BP_NPC_C|GetActivate%20Input (Variables|Default|GetNPC)))
          (Class|BPINpcInteractable|Interact(Message) (Variables|Default|GetInteractable%20Npc) _self)
          (Pawn|Components|CharacterMovement|SetMovementMode (Variables|Character|GetCharacterMovement _self) "MOVE_None" 0)
          (if (Variables|/Game/Blueprints/NPC/BP_NPC.BP_NPC_C|GetMove%20player (Variables|Default|GetNPC))
            (Transformation|SetActorLocationAndRotation (Variables|/Game/Blueprints/NPC/BP_NPC.BP_NPC_C|GetPlayerPosition _npc) (Variables|/Game/Blueprints/NPC/BP_NPC.BP_NPC_C|GetPlayerRotation _npc))))))))

(event Input|EnhancedActionEvents|EnhancedInputActionIA_SkipDialogue
  (params (ActionValue :type Boolean) (ElapsedSeconds :type Float%20%28double-precision%29) (TriggeredSeconds :type Float%20%28double-precision%29) (InputAction :type Input%20Action%20Object%20Reference :default "/Game/Inputs/IA_SkipDialogue.IA_SkipDialogue"))
  (:Started
    (Class|BPINpcInteractable|SkipDialogue(Message) (Variables|Default|GetInteractable%20Npc))))

(event EventClearReferences
  (Variables|/Game/Blueprints/NPC/BP_NPC.BP_NPC_C|SetActivate%20Input (Variables|Default|GetNPC) false)
  (Variables|Default|SetInteractable%20Npc 0)
  (Variables|Default|SetNPC 0)
  (Pawn|Components|CharacterMovement|SetMovementMode (Variables|Character|GetCharacterMovement) "MOVE_Walking" 0)
  (Game|Player|SetViewTargetwithBlend (Game|GetPlayerController 0) (Components|GetOwner (Variables|Default|GetCamera)) 0.0 "VTBlend_Linear" 0.0 false))

(event EventZoomTransition
  (Utilities|FlowControl|Delay 0.5)
  (Utilities|Struct|SetmembersinPostProcessSettings (Variables|/Script/Engine.CameraComponent|GetPostProcessSettings (Variables|Default|GetCamera)) 0.0)
  (bind _lerp_fov (Timeline|Zoom%20Timeline PlayFromStart)
    (:Update
      (Camera|SetFieldOfView (Variables|Default|GetCamera) _lerp_fov))
    (:Finished
      (Utilities|FlowControl|Delay 2.0)
      (Utilities|Struct|SetmembersinPostProcessSettings (Variables|/Script/Engine.CameraComponent|GetPostProcessSettings (Variables|Default|GetCamera)) 1.2e+03))))

(fn ConstructionScript)