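; Battle manager for an Undertale-style encounter that randomly picks a rock or frog enemy data asset and runs its dialogue, fight and death scenes.
; HandleState switches on the current state to drive dialogue, combat and teardown, using Fight, Talk and Mercy widgets.
; Timelines scale the battle box up for dialogue, down for the player's heart phase, and fade out defeated enemies.
; Skip input advances dialogue arrays, then shrinks the box or ends the battle.
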(event Custom|Increase%20Box%20for%20enemy%20death
  (bind _skipwidget (Variables|Default|GetSkipWidget))
  (bind _enemyda (Variables|Default|GetEnemyDA))
  (bind _enemydata (Variables|/Game/Blueprints/Battles/Enemies/DA_EnemyData.DA_EnemyData_C|GetEnemyData _enemyda))
  ;[1 0.8962 0.5284] Increase Box for enemy death
  (Variables|Default|SetDialogue%20count 3)
  (Variables|Default|SetCurrentState "NewEnumerator4")
  (Variables|Default|SetReduced false)
  (bind _enemy (Variables|Default|GetEnemy)
    (:then
      (switch string (.name _enemydata)
        (:Chill%20Rock
          (Rendering|Components|Sprite|SetSprite (Variables|/Game/Blueprints/Battles/Enemies/BP_Enemy.BP_Enemy_C|GetPaperSprite (Variables|Default|GetEnemy)) (Utilities|Array|Get(acopy) (.sprite _enemydata)))
          (bind _scale_lerp (Timeline|Timeline_0 PlayFromStart)
            (:Update
              (Transformation|SetActorScale3D (Variables|Default|GetBattleBox) (Math|Vector|Lerp(Vector) "0.750000,0.750000,1.000000" "1.000000,2.500000,1.000000" _scale_lerp)))
            (:Finished
              (CallFunction|HandleState)
              (UserInterface|Viewport|AddtoViewport (Variables|Default|GetDialogueWidget) 0)
              (UserInterface|Viewport|AddtoViewport _skipwidget 0)
              (Default|FlickerEvent _skipwidget)
              (bind _vanish (Timeline|Vanish%20enemy PlayFromStart)
                (:Update
                  (Rendering|Material|SetScalarParameterValueonMaterials (Variables|/Game/Blueprints/Battles/Enemies/BP_Enemy.BP_Enemy_C|GetPaperSprite (Variables|Default|GetEnemy)) "Opacity" _vanish))))))
        (:Frog
          (Sprite|SetFlipbook (Variables|/Game/Blueprints/Battles/Enemies/BP_Enemy.BP_Enemy_C|GetPaperFlipbook _enemy))
          (Rendering|Components|Sprite|SetSprite (Variables|/Game/Blueprints/Battles/Enemies/BP_Enemy.BP_Enemy_C|GetPaperSprite (Variables|Default|GetEnemy)) "/Game/Sprite/Frog/T_frog_Sprite_2.T_frog_Sprite_2")
          (Timeline|Timeline_0 PlayFromStart))))
    (:else)))

(event Custom|Increaese_box_size
  (bind _skipwidget (Variables|Default|GetSkipWidget))
  (bind _enemyda (Variables|Default|GetEnemyDA))
  (bind _enemydata (Variables|/Game/Blueprints/Battles/Enemies/DA_EnemyData.DA_EnemyData_C|GetEnemyData _enemyda))
  ;[1 0.7562 0.5386] INCREASE BOX
  (Variables|Default|SetReduced false)
  (bind _enemy (Variables|Default|GetEnemy)
    (:then
      (switch string (.name _enemydata)
        (:Chill%20Rock
          (Rendering|Components|Sprite|SetSprite (Variables|/Game/Blueprints/Battles/Enemies/BP_Enemy.BP_Enemy_C|GetPaperSprite (Variables|Default|GetEnemy)) (Utilities|Array|Get(acopy) (.sprite _enemydata)))
          (bind _scale_lerp (Timeline|increase%20box%20size PlayFromStart)
            (:Update
              (Transformation|SetActorScale3D (Variables|Default|GetBattleBox) (Math|Vector|Lerp(Vector) "0.750000,0.750000,1.000000" "1.000000,2.500000,1.000000" _scale_lerp)))
            (:Finished
              (UserInterface|Viewport|AddtoViewport (Variables|Default|GetDialogueWidget) 0)
              (UserInterface|Viewport|AddtoViewport _skipwidget 0)
              (Default|FlickerEvent _skipwidget))))
        (:Frog
          (Sprite|SetFlipbook (Variables|/Game/Blueprints/Battles/Enemies/BP_Enemy.BP_Enemy_C|GetPaperFlipbook _enemy) (.paperflipbook _enemydata))
          (Rendering|Components|Sprite|SetSprite (Variables|/Game/Blueprints/Battles/Enemies/BP_Enemy.BP_Enemy_C|GetPaperSprite (Variables|Default|GetEnemy)) 0)
          (Timeline|increase%20box%20size PlayFromStart))))
    (:else)))

(event Custom|Reduce_box_size
  (bind _normalplayer (Variables|Default|GetNormalPlayer))
  ;[0.4579 1 0.9801] REDUCE BOX
  (if (not (Variables|Default|GetReduced))
    (Widget|RemovefromParent (Variables|Default|GetDialogueWidget))
    (bind _scale_lerp (Timeline|Timeline PlayFromStart)
      (:Update
        (Transformation|SetActorScale3D (Variables|Default|GetBattleBox) (Math|Vector|Lerp(Vector) "1.000000,2.500000,1.000000" "0.750000,0.750000,1.000000" _scale_lerp)))
      (:Finished
        (Default|InteractableFight (Variables|Default|GetFightButton))
        (Default|InteractableTalk (Variables|Default|GetTalkButton))
        (if (Variables|Default|GetSpawned)
          _
          (else
            (Class|MyPlayerCharacter|SpawnHeart _normalplayer)
            (Variables|Default|SetSpawned true)))
        (Class|MyPlayerCharacter|ShowHeart _normalplayer)
        (Variables|Default|SetReduced true)))))

(event Input|EnhancedActionEvents|EnhancedInputActionIA_SkipDialogue
  (params (ActionValue :type Boolean) (ElapsedSeconds :type Float%20%28double-precision%29) (TriggeredSeconds :type Float%20%28double-precision%29) (InputAction :type Input%20Action%20Object%20Reference :default "/Game/Inputs/IA_SkipDialogue.IA_SkipDialogue"))
  ;[1 0.4272 0.1094] SKIP DIALOGUE
  (:Started
    (if (Variables|Default|GetXActive)
      (switch int (Variables|Default|GetDialogue%20count)
        (:1
          (CallFunction|SkipDialogue (.firstdialogue (Variables|/Game/Blueprints/Battles/Enemies/DA_EnemyData.DA_EnemyData_C|GetEnemyData (Variables|Default|GetEnemyDA)))))
        (:2
          (CallFunction|SkipDialogue (.2nddialogue (Variables|/Game/Blueprints/Battles/Enemies/DA_EnemyData.DA_EnemyData_C|GetEnemyData (Variables|Default|GetEnemyDA)))))
        (:3
          (CallFunction|SkipDialogue (.deathdialogue (Variables|/Game/Blueprints/Battles/Enemies/DA_EnemyData.DA_EnemyData_C|GetEnemyData (Variables|Default|GetEnemyDA)))))))))

(event EventBeginPlay
  ;[1 1 1] BEGIN SETUP
  (bind _returnvalue (UserInterface|CreateWidget "/Game/UI/Combat/WB_Dialogue.WB_Dialogue_C"))
  (Variables|Default|SetDialogueWidget _returnvalue)
  (bind _returnvalue_2 (UserInterface|CreateWidget "/Game/UI/Combat/WB_TriangleDialogue.WB_TriangleDialogue_C"))
  (Variables|Default|SetSkipWidget _returnvalue_2)
  (bind _returnvalue_3 (UserInterface|CreateWidget "/Game/UI/Combat/WB_TalkButton.WB_TalkButton_C"))
  (Variables|Default|SetTalkButton _returnvalue_3)
  (bind _returnvalue_4 (UserInterface|CreateWidget "/Game/UI/Combat/WB_FightButton.WB_FightButton_C"))
  (Variables|Default|SetFightButton _returnvalue_4)
  (bind _returnvalue_5 (UserInterface|CreateWidget "/Game/UI/Combat/WB_MercyButton.WB_MercyButton_C"))
  (Variables|Default|SetMercyButton _returnvalue_5)
  (bind _returnvalue_6 (UserInterface|CreateWidget "/Game/UI/Combat/WB_MercyNotActive.WB_MercyNotActive_C"))
  (Variables|Default|SetNotActiveMercy _returnvalue_6)
  (Input|EnableInput (Game|GetPlayerController 0))
  (bind _outactors (Actor|GetAllActorsOfClasswithTag "/Game/Blueprints/MainCharacter/NormalPlayer/BP_PlayerCharacter.BP_PlayerCharacter_C" "Player Character"))
  (Variables|Default|SetNormalPlayer (Utilities|Array|Get(acopy) _outactors)))

(fn ConstructionScript)

(fn HandleState
  (switch Utilities|FlowControl|Switch|SwitchonE_BattleEvent (Variables|Default|GetCurrentState)
    (:NewEnumerator0
      (switch int (Math|Random|RandomInteger 2)
        (:0
          (Variables|Default|SetEnemyDA "/Game/Blueprints/Battles/Enemies/DA_Rock.DA_Rock"))
        (:1
          (Variables|Default|SetEnemyDA "/Game/Blueprints/Battles/Enemies/DA_Frog.DA_Frog")))
      (CallFunction|StartFirstDialogue))
    (:NewEnumerator1
      (CallFunction|StartBattle))
    (:NewEnumerator2
      (CallFunction|StartSecondDialogue))
    (:NewEnumerator3
      (CallFunction|EndBattle))
    (:NewEnumerator4
      (CallFunction|EnemyDeathScene))))

(fn StartFirstDialogue
  (Variables|Default|SetExiting%20for%20death false)
  (UserInterface|Viewport|AddtoViewport (Variables|Default|GetFightButton) 0)
  (UserInterface|Viewport|AddtoViewport (Variables|Default|GetTalkButton) 0)
  (UserInterface|Viewport|AddtoViewport (Variables|Default|GetNotActiveMercy) 0)
  (CallFunction|IncreaeseBoxSize)
  (Variables|Default|SetDialogue%20index 0)
  (Default|UpdateDialogue (Variables|Default|GetDialogueWidget) (Utilities|Array|Get(acopy) (.firstdialogue (Variables|/Game/Blueprints/Battles/Enemies/DA_EnemyData.DA_EnemyData_C|GetEnemyData (Variables|Default|GetEnemyDA))) (Variables|Default|GetDialogue%20index)))
  (Variables|Default|SetXActive true))

(fn StartBattle
  (bind _normalplayer (Variables|Default|GetNormalPlayer))
  (Input|SetInputModeGameOnly (Game|GetPlayerController 0) false)
  (Variables|Default|SetXActive false)
  (if (Variables|Default|GetReduced)
    _
    (else
      (CallFunction|ReduceBoxSize)
      (Variables|Default|SetReduced true)))
  (if (Variables|Default|GetSpawned)
    _
    (else
      (Class|MyPlayerCharacter|SpawnHeart _normalplayer)
      (Variables|Default|SetSpawned true)))
  (Class|MyPlayerCharacter|ShowHeart _normalplayer)
  (Default|StartFight (Variables|Default|GetEnemy) (.name (Variables|/Game/Blueprints/Battles/Enemies/DA_EnemyData.DA_EnemyData_C|GetEnemyData (Variables|Default|GetEnemyDA)))))

(fn RemoveDialogue
  (Widget|RemovefromParent (Variables|Default|GetDialogueWidget)))

(fn EndBattle
  (bind _enemy (Variables|Default|GetEnemy))
  (Variables|Default|SetSpawned false)
  (Variables|Default|SetDialogue%20index 0)
  (Variables|Default|SetDialogue%20count 1)
  (Variables|Default|SetCurrentState "NewEnumerator0")
  (Input|SetInputModeGameOnly (Game|GetPlayerController 0) false)
  (Sprite|SetFlipbook (Variables|/Game/Blueprints/Battles/Enemies/BP_Enemy.BP_Enemy_C|GetPaperFlipbook _enemy))
  (Rendering|Components|Sprite|SetSprite (Variables|/Game/Blueprints/Battles/Enemies/BP_Enemy.BP_Enemy_C|GetPaperSprite _enemy) 0)
  (Widget|RemovefromParent (Variables|Default|GetFightButton))
  (Widget|RemovefromParent (Variables|Default|GetMercyButton))
  (Widget|RemovefromParent (Variables|Default|GetNotActiveMercy))
  (Widget|RemovefromParent (Variables|Default|GetTalkButton))
  (Class|MyPlayerCharacter|ExitCombat (Variables|Default|GetNormalPlayer)))

(fn SkipDialogue
  (params (Dialogue%20Array :type Array%20of%20Texts))
  (Variables|Default|SetDialogue%20index (+ 1 (Variables|Default|GetDialogue%20index)))
  (if (== (Utilities|Array|Length Dialogue%20Array) (Variables|Default|GetDialogue%20index))
    (Widget|RemovefromParent (Variables|Default|GetSkipWidget))
    (Math|Integer|IncrementInt (Variables|Default|GetDialogue%20count)
      (:%20%20
        (if (Variables|Default|GetExiting%20for%20death)
          (Widget|RemovefromParent (Variables|Default|GetDialogueWidget))
          (Variables|Default|SetCurrentState "NewEnumerator3")
          (CallFunction|HandleState)
          (else
            (CallFunction|ReduceBoxSize)))))
    (else
      (Default|UpdateDialogue (Variables|Default|GetDialogueWidget) (Utilities|Array|Get(acopy) Dialogue%20Array (Variables|Default|GetDialogue%20index)))
      (Default|Pressed (Variables|Default|GetSkipWidget)))))

(fn UnfocusWidget
  (Input|SetInputModeGameOnly (Game|GetPlayerController 0) false))

(fn StartSecondDialogue
  (Class|MyPlayerCharacter|HideHeart (Variables|Default|GetNormalPlayer))
  (CallFunction|IncreaeseBoxSize)
  (Variables|Default|SetDialogue%20index 0)
  (Default|UpdateDialogue (Variables|Default|GetDialogueWidget) (Utilities|Array|Get(acopy) (.2nddialogue (Variables|/Game/Blueprints/Battles/Enemies/DA_EnemyData.DA_EnemyData_C|GetEnemyData (Variables|Default|GetEnemyDA))) (Variables|Default|GetDialogue%20index)))
  (Variables|Default|SetXActive true))

(fn StartTalking
  (Default|Talk (Variables|Default|GetEnemy) (.name (Variables|/Game/Blueprints/Battles/Enemies/DA_EnemyData.DA_EnemyData_C|GetEnemyData (Variables|Default|GetEnemyDA)))))

(fn EnemyDeathScene
  (Variables|Default|SetExiting%20for%20death true)
  (Variables|Default|SetDialogue%20index 0)
  (Default|UpdateDialogue (Variables|Default|GetDialogueWidget) (Utilities|Array|Get(acopy) (.deathdialogue (Variables|/Game/Blueprints/Battles/Enemies/DA_EnemyData.DA_EnemyData_C|GetEnemyData (Variables|Default|GetEnemyDA))) (Variables|Default|GetDialogue%20index)))
  (Variables|Default|SetXActive true))