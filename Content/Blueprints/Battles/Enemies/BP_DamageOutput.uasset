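; Floating damage text actor for enemy battles that shows a damage value, drifts, then removes itself.
; On BeginPlay it passes DamageOutput to the WB_DamageTxt widget in its DmgText component and plays the MoveDmgText timeline.
; Each timeline update shifts it along negative X and Y from its current location, so movement accumulates per frame, with Z unchanged.
; The actor destroys itself when the timeline finishes.
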(event EventBeginPlay
  (bind _returnvalue (Transformation|GetActorLocation))
  (bind _xy_distance (Variables|Default|GetXY%20Distance))
  (bind _aswb_damage_txt (Utilities|Casting|CastToWB_DamageTxt (UserInterface|GetWidget (Variables|Default|GetDmgText))))
  (Variables|/Game/UI/Combat/WB_DamageTxt.WB_DamageTxt_C|SetDamage%20Output _aswb_damage_txt (Variables|Default|GetDamage%20Output))
  (bind _move_txt (Timeline|Move%20dmg%20text PlayFromStart)
    (:Update
      (Transformation|SetActorLocation (Math|Vector|Lerp(Vector) (Transformation|GetActorLocation) (Math|Vector|MakeVector (- (.x _returnvalue) _xy_distance) (- (.y _returnvalue) _xy_distance) (.z _returnvalue)) _move_txt) false false))
    (:Finished
      (Actor|DestroyActor))))

(fn ConstructionScript)