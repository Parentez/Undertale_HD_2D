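; Battle enemy actor (Chill Rock or Frog) that alternates the player's timed-hit attack with its own projectile attack sequences.
; StartFight shows the damage UI and spawns a moving bar; IA_DealDamage stops it, and overlapped hit zones scale randomized damage.
; If the enemy survives, name-based sequencers run delay-timed spawner patterns, then hand state back to BattleManager.
; Death triggers the battle box transition; CheckForNoEnemy tallies per-area kills to update battle state.
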(event Custom|Rock%20Sequencer
  (params (Sequence%20Number :type Integer))
  (bind _battlemanager (Variables|Default|GetBattleManager))
  ;[0.3753 0.5276 0.9844] Rock
  ;;[0.9468 1 0.9341] Sequence 1
  (Rendering|Components|Sprite|SetSprite (Variables|Default|GetPaperSprite) (Utilities|Array|Get(acopy) (.sprite (Variables|/Game/Blueprints/Battles/Enemies/DA_EnemyData.DA_EnemyData_C|GetEnemyData (Variables|/Game/Blueprints/Battles/BP_BattleManager.BP_BattleManager_C|GetEnemyDA (Variables|Default|GetBattleManager)))) 1))
  (switch int Sequence%20Number
    (:1
      (Utilities|FlowControl|Delay 1.5)
      (Class|ProjectileSpawnerComponent|FallingRocks (Variables|/Game/Blueprints/Projectiles/BP_Spawner.BP_Spawner_C|GetProjectileSpawner (Variables|Spawners|GetSpawner%204)) 6e+02 30 1e+01)
      (Utilities|FlowControl|Delay 12.0)
      (Math|Integer|IncrementInt (Variables|Default|GetSequence%20count)
        (:%20%20
          (if (Variables|Default|Get2ndDialogueDone)
            (Variables|/Game/Blueprints/Battles/BP_BattleManager.BP_BattleManager_C|SetCurrentState _battlemanager "NewEnumerator1")
            (else
              (Variables|/Game/Blueprints/Battles/BP_BattleManager.BP_BattleManager_C|SetCurrentState _battlemanager "NewEnumerator2")
              (Variables|Default|Set2ndDialogueDone true)))
          (Default|HandleState (Variables|Default|GetBattleManager)))))
    (:2
      ;;[1 1 1] Sequence 2
      (Utilities|FlowControl|Delay 1.5)
      (Class|ProjectileSpawnerComponent|FallingRocks (Variables|/Game/Blueprints/Projectiles/BP_Spawner.BP_Spawner_C|GetProjectileSpawner (Variables|Spawners|GetSpawner%204)) 6e+02 25 8.0)
      (Utilities|FlowControl|Delay 1e+01)
      (Variables|/Game/Blueprints/Battles/BP_BattleManager.BP_BattleManager_C|SetCurrentState (Variables|Default|GetBattleManager) "NewEnumerator1")
      (Default|HandleState (Variables|Default|GetBattleManager))
      (Variables|Default|SetSequence%20count 1))))

(event Custom|Rock%20Player%20death
  ;[0.3753 0.5276 0.9844] Rock
)

(event Custom|Frog%20Sequencer
  (params (Sequence%20Number :type Integer))
  (bind _enemy_location (Variables|Default|Getenemy%20location))
  (bind _battlemanager (Variables|Default|GetBattleManager))
  ;[0.6421 1 0.5684] Frog
  (Sprite|SetFlipbook (Variables|Default|GetPaperFlipbook))
  (Rendering|Components|Sprite|SetSprite (Variables|Default|GetPaperSprite) (Utilities|Array|Get(acopy) (.sprite (Variables|/Game/Blueprints/Battles/Enemies/DA_EnemyData.DA_EnemyData_C|GetEnemyData (Variables|/Game/Blueprints/Battles/BP_BattleManager.BP_BattleManager_C|GetEnemyDA (Variables|Default|GetBattleManager))))))
  (Transformation|SetActorLocation (Math|Vector|MakeVector (+ (.x _enemy_location) 3e+02) (.y _enemy_location) (.z _enemy_location)) false false)
  (switch int Sequence%20Number
    (:1
      (Utilities|FlowControl|Delay 1.5)
      (Class|ProjectileSpawnerComponent|FrogTongue (Variables|/Game/Blueprints/Projectiles/BP_Spawner.BP_Spawner_C|GetProjectileSpawner (Variables|Spawners|GetSpawner2)) "0.000000,-1.000000,0.000000" 4e+02 1)
      (Utilities|FlowControl|Delay 2.0)
      (Class|ProjectileSpawnerComponent|FrogTongue (Variables|/Game/Blueprints/Projectiles/BP_Spawner.BP_Spawner_C|GetProjectileSpawner (Variables|Spawners|GetSpawner1)) "0.000000,1.000000,0.000000" 2e+02 1)
      (Utilities|FlowControl|Delay 1.0)
      (Class|ProjectileSpawnerComponent|FrogTongue (Variables|/Game/Blueprints/Projectiles/BP_Spawner.BP_Spawner_C|GetProjectileSpawner (Variables|Spawners|GetSpawner3)) "1.000000,0.000000,0.000000" 4e+02 0 1)
      (Utilities|FlowControl|Delay 5.0)
      (Math|Integer|IncrementInt (Variables|Default|GetSequence%20count)
        (:%20%20
          (if (Variables|Default|Get2ndDialogueDone)
            (Variables|/Game/Blueprints/Battles/BP_BattleManager.BP_BattleManager_C|SetCurrentState _battlemanager "NewEnumerator1")
            (else
              (Variables|/Game/Blueprints/Battles/BP_BattleManager.BP_BattleManager_C|SetCurrentState _battlemanager "NewEnumerator2")
              (Variables|Default|Set2ndDialogueDone true)))
          (Sprite|SetFlipbook (Variables|Default|GetPaperFlipbook) (.paperflipbook (Variables|/Game/Blueprints/Battles/Enemies/DA_EnemyData.DA_EnemyData_C|GetEnemyData (Variables|/Game/Blueprints/Battles/BP_BattleManager.BP_BattleManager_C|GetEnemyDA (Variables|Default|GetBattleManager)))))
          (Rendering|Components|Sprite|SetSprite (Variables|Default|GetPaperSprite) 0)
          (Transformation|SetActorLocation (Variables|Default|Getenemy%20location) false false)
          (Default|HandleState (Variables|Default|GetBattleManager)))))
    (:2
      (Utilities|FlowControl|Delay 1.5)
      (Class|ProjectileSpawnerComponent|FrogTongue (Variables|/Game/Blueprints/Projectiles/BP_Spawner.BP_Spawner_C|GetProjectileSpawner (Variables|Spawners|GetSpawner1)) "0.000000,1.000000,0.000000" 2e+02 1)
      (Utilities|FlowControl|Delay 1.0)
      (Class|ProjectileSpawnerComponent|FrogTongue (Variables|/Game/Blueprints/Projectiles/BP_Spawner.BP_Spawner_C|GetProjectileSpawner (Variables|Spawners|GetSpawner3)) "1.000000,0.000000,0.000000" 4e+02 0 1)
      (Utilities|FlowControl|Delay 1.0)
      (Class|ProjectileSpawnerComponent|FrogTongue (Variables|/Game/Blueprints/Projectiles/BP_Spawner.BP_Spawner_C|GetProjectileSpawner (Variables|Spawners|GetSpawner2)) "0.000000,-1.000000,0.000000" 4e+02 1)
      (Utilities|FlowControl|Delay 5.0)
      (Variables|/Game/Blueprints/Battles/BP_BattleManager.BP_BattleManager_C|SetCurrentState (Variables|Default|GetBattleManager) "NewEnumerator1")
      (Sprite|SetFlipbook (Variables|Default|GetPaperFlipbook) (.paperflipbook (Variables|/Game/Blueprints/Battles/Enemies/DA_EnemyData.DA_EnemyData_C|GetEnemyData (Variables|/Game/Blueprints/Battles/BP_BattleManager.BP_BattleManager_C|GetEnemyDA (Variables|Default|GetBattleManager)))))
      (Rendering|Components|Sprite|SetSprite (Variables|Default|GetPaperSprite) 0)
      (Transformation|SetActorLocation (Variables|Default|Getenemy%20location) false false)
      (Default|HandleState (Variables|Default|GetBattleManager))
      (Variables|Default|SetSequence%20count 1))))

(event Custom|Enable%20Damage%20bar
  ;[1 1 1] Activate Damage attack
  (switch string (.name (Variables|/Game/Blueprints/Battles/Enemies/DA_EnemyData.DA_EnemyData_C|GetEnemyData (Variables|/Game/Blueprints/Battles/BP_BattleManager.BP_BattleManager_C|GetEnemyDA (Variables|Default|GetBattleManager))))
    (:Chill%20Rock
      (Variables|Default|Setmax%20bars 1)
      (bind _returnvalue (Game|SpawnActorfromClass "/Game/Blueprints/Contestual/BP_Bar.BP_Bar_C" (Math|Transform|MakeTransform "-942.822101,6400.000000,200.000000" "0.000000,-90.000000,90.000000" "1.000000,1.000000,0.800000") "Undefined" "MultiplyWithRoot" 0 0))
      (Utilities|Array|Add (Variables|Default|GetSpawned%20Bars) _returnvalue))
    (:Frog
      (Variables|Default|Setmax%20bars 1)
      (bind _returnvalue_2 (Game|SpawnActorfromClass "/Game/Blueprints/Contestual/BP_Bar.BP_Bar_C" (Math|Transform|MakeTransform "-942.822101,6400.000000,200.000000" "0.000000,-90.000000,90.000000" "1.000000,1.000000,0.800000") "Undefined" "MultiplyWithRoot" 0 0))
      (Utilities|Array|Add (Variables|Default|GetSpawned%20Bars) _returnvalue_2))))

(event Custom|Start%20Damage%20bar
  (bind _damageui (Variables|Default|GetDamageUI))
  ;[1 1 1] Activate Damage attack
  (Variables|Default|SetEnemyDeath false)
  (Class|MyPlayerCharacter|HideHeart (Variables|/Game/Blueprints/Battles/BP_BattleManager.BP_BattleManager_C|GetNormalPlayer (Variables|Default|GetBattleManager)))
  (Rendering|SetActorHiddenInGame (Variables|Default|GetBattlebox) true)
  (Default|ShowDamageDealer _damageui)
  (EventDispatchers|BindEventtoOnIncreaseFinished _damageui (delegate Custom|Enable%20Damage%20bar)))

(event Custom|Back%20to%20normal%20combat%20scene
  ;[0.9987 1 0.9767] Damage Logic
  (if (not (Variables|Default|GetEnemyDeath))
    (Rendering|SetActorHiddenInGame (Variables|Default|GetBattlebox) false)
    (CallFunction|StartSequncer (Variables|Default|GetEnemy%20Name))
    (Class|MyPlayerCharacter|ShowHeart (Variables|/Game/Blueprints/Battles/BP_BattleManager.BP_BattleManager_C|GetNormalPlayer (Variables|Default|GetBattleManager)))))

(event Custom|Enemy%20death%20call
  ;[0.9987 1 0.9767] Damage Logic
  (if (Variables|Default|GetEnemyDeath)
    (Rendering|SetActorHiddenInGame (Variables|Default|GetBattlebox) false)
    (Default|IncreaseBoxforEnemyDeath (Variables|Default|GetBattleManager))))

(event Custom|Remove%20Bar%20From%20array
  (params (Bar :type BP%20Bar%20Object%20Reference))
  ;[1 0.9965 0.6731] Destroy bar if not pressed
  (Utilities|Array|RemoveItem (Variables|Default|GetSpawned%20Bars) Bar)
  (Actor|DestroyActor Bar)
  (Math|Integer|DecrementInt (Variables|Default|Getmax%20bars)
    (:%20%20
      (if (== (Utilities|Array|Length (Variables|Default|GetSpawned%20Bars)) (Variables|Default|Getmax%20bars))
        ;[0.9987 1 0.9767] Damage Logic
        (Variables|Default|Setbars%20count 0)
        (Utilities|Array|Clear (Variables|Default|GetSpawned%20Bars))
        (Utilities|FlowControl|Delay 1.5)
        (Actor|DestroyActor (Variables|Default|Getspawned%20bar))
        (Default|HideDamageDealer (Variables|Default|GetDamageUI))
        (EventDispatchers|AssignOnDecreaseFinished (Variables|Default|GetDamageUI) (delegate Custom|Back%20to%20normal%20combat%20scene))))))

(event Input|EnhancedActionEvents|EnhancedInputActionIA_DealDamage
  (params (ActionValue :type Boolean) (ElapsedSeconds :type Float%20%28double-precision%29) (TriggeredSeconds :type Float%20%28double-precision%29) (InputAction :type Input%20Action%20Object%20Reference :default "/Game/Inputs/IA_DealDamage.IA_DealDamage"))
  (bind _returnvalue (Transformation|GetActorLocation))
  (bind _damageui (Variables|Default|GetDamageUI))
  (bind _spawned_bars (Variables|Default|GetSpawned%20Bars))
  ;[0.9987 1 0.9767] Damage Logic
  (:Started
    (if (!= (Utilities|Array|Length (Variables|Default|GetSpawned%20Bars)) 0)
      (bind _output_get (Variables|Default|Setspawned%20bar (Utilities|Array|Get(acopy) (Variables|Default|GetSpawned%20Bars) (Variables|Default|Getbars%20count))))
      (Default|StopMovement _output_get)
      (Variables|Default|SetEnemy%20hit false)
      (bind _keys (Utilities|Map|Keys (Variables|/Game/Blueprints/Contestual/BP_DamageUI.BP_DamageUI_C|GetHitZones (Variables|Default|GetDamageUI))))
      (for _array_element _keys
        (Utilities|IsValid _array_element
          (:Is%20Valid
            (if (Collision|IsOverlappingActor _array_element (Utilities|Array|Get(acopy) (Variables|Default|GetSpawned%20Bars) (Variables|Default|Getbars%20count)) :!class /Script/Engine.PrimitiveComponent)
              (Variables|Default|SetBarMultiplier _array_element)
              (Variables|Default|SetEnemy%20hit true)))))
      (if (Variables|Default|GetEnemy%20hit)
        (Game|SpawnActorfromClass "/Game/Blueprints/Battles/Enemies/BP_DamageOutput.BP_DamageOutput_C" (Math|Transform|MakeTransform (Math|Vector|MakeVector (+ (.x _returnvalue) 1e+02) (+ (.y _returnvalue) 2e+02) (.z _returnvalue)) "0, 0, 0" "4.000000,4.000000,4.000000") "Undefined" "MultiplyWithRoot" 0 -2.0 (Math|Float|Truncate (* (.Value (Utilities|Map|Find (Variables|/Game/Blueprints/Contestual/BP_DamageUI.BP_DamageUI_C|GetHitZones (Variables|Default|GetDamageUI)) (Variables|Default|GetBarMultiplier))) (+ (+ (Math|Random|RandomInteger 20) 1) (Variables|/Script/Undertale_HD_2D.MyPlayerCharacter|GetPlayerAtkDmg (Variables|/Game/Blueprints/Battles/BP_BattleManager.BP_BattleManager_C|GetNormalPlayer (Variables|Default|GetBattleManager)))))) "" 0)
        (bind _output_get_2 (Variables|Default|SetEnemy%20HP (- (Variables|Default|GetEnemy%20HP) (Math|Float|Truncate (* (.Value (Utilities|Map|Find (Variables|/Game/Blueprints/Contestual/BP_DamageUI.BP_DamageUI_C|GetHitZones (Variables|Default|GetDamageUI)) (Variables|Default|GetBarMultiplier))) (+ (+ (Math|Random|RandomInteger 20) 1) (Variables|/Script/Undertale_HD_2D.MyPlayerCharacter|GetPlayerAtkDmg (Variables|/Game/Blueprints/Battles/BP_BattleManager.BP_BattleManager_C|GetNormalPlayer (Variables|Default|GetBattleManager)))))))))
        (if (<= _output_get_2 0)
          (Variables|Default|SetEnemyDeath true)
          (Variables|Default|SetEnemy%20HP -1000)
          (Actor|DestroyActor (Utilities|Array|Get(acopy) _spawned_bars))
          (Utilities|Array|Clear _spawned_bars)
          (Default|HideDamageDealer _damageui)
          (Variables|Default|SetSequence%20count 1)
          (Variables|Default|Setbars%20count 0)
          (EventDispatchers|AssignOnDecreaseFinished _damageui (delegate Custom|Enemy%20death%20call))
          (else
            (Math|Integer|IncrementInt (Variables|Default|Getbars%20count) :!label _label
              (:%20%20
                (if (== (Utilities|Array|Length (Variables|Default|GetSpawned%20Bars)) (Variables|Default|Getmax%20bars))
                  (Variables|Default|Setbars%20count 0)
                  (Utilities|Array|Clear (Variables|Default|GetSpawned%20Bars))
                  (Utilities|FlowControl|Delay 1.5)
                  (Actor|DestroyActor (Variables|Default|Getspawned%20bar))
                  (Default|HideDamageDealer (Variables|Default|GetDamageUI))
                  (EventDispatchers|AssignOnDecreaseFinished (Variables|Default|GetDamageUI) (delegate Custom|Back%20to%20normal%20combat%20scene)))))))
        (else
          (Game|SpawnActorfromClass "/Game/Blueprints/Battles/Enemies/BP_DamageOutput.BP_DamageOutput_C" (Math|Transform|MakeTransform (Transformation|GetActorLocation) "0, 0, 0" "4.000000,4.000000,4.000000") "Undefined" "MultiplyWithRoot" 0 -2.0 0 "MISS" 0)
          (goto _label))))))

(event EventBeginPlay
  ;[1 0.3281 0.3281] Enable space bar input
  (Input|EnableInput (Game|GetPlayerController 0))
  (Variables|Default|Setenemy%20location (Transformation|GetActorLocation)))

(fn ConstructionScript)

(fn StartFight
  (params (Enemy%20name :type String))
  (Variables|Default|SetEnemy%20Name Enemy%20name)
  (CallFunction|StartDamageBar)
  (if (== (Variables|Default|GetEnemy%20HP) -1000)
    (Variables|Default|Set2ndDialogueDone false)
    (Variables|Default|SetEnemy%20HP (.enemyhp (Variables|/Game/Blueprints/Battles/Enemies/DA_EnemyData.DA_EnemyData_C|GetEnemyData (Variables|/Game/Blueprints/Battles/BP_BattleManager.BP_BattleManager_C|GetEnemyDA (Variables|Default|GetBattleManager)))))))

(fn StartSequncer
  (params (Enemy%20name :type String))
  (switch string Enemy%20name
    (:Chill%20Rock
      (CallFunction|RockSequencer (Variables|Default|GetSequence%20count)))
    (:Frog
      (CallFunction|FrogSequencer (Variables|Default|GetSequence%20count)))))

(fn CheckforNoEnemy
  (bind _battlemanager (Variables|Default|GetBattleManager))
  (bind _battlemanager_2 (Variables|Default|GetBattleManager))
  (bind _battlemanager_3 (Variables|Default|GetBattleManager))
  (bind _normalplayer (Variables|/Game/Blueprints/Battles/BP_BattleManager.BP_BattleManager_C|GetNormalPlayer _battlemanager))
  (bind _normalplayer_2 (Variables|/Game/Blueprints/Battles/BP_BattleManager.BP_BattleManager_C|GetNormalPlayer _battlemanager_3))
  (bind _normalplayer_3 (Variables|/Game/Blueprints/Battles/BP_BattleManager.BP_BattleManager_C|GetNormalPlayer _battlemanager_2))
  (bind _enemieskilledarea2 (Variables|/Script/Undertale_HD_2D.MyPlayerCharacter|GetEnemiesKilledArea2 _normalplayer_2))
  (if (Variables|/Game/Blueprints/Battles/BP_BattleManager.BP_BattleManager_C|GetFigthed (Variables|Default|GetBattleManager))
    (if (.inarea1 (Variables|/Game/Blueprints/Battles/Enemies/DA_EnemyData.DA_EnemyData_C|GetEnemyData (Variables|/Game/Blueprints/Battles/BP_BattleManager.BP_BattleManager_C|GetEnemyDA (Variables|Default|GetBattleManager))))
      (bind _result (Math|Integer|IncrementInt (Variables|/Script/Undertale_HD_2D.MyPlayerCharacter|GetEnemiesKilledArea1 _normalplayer_2))
        (:%20%20
          (Development|PrintText (Utilities|Text|ToText(Integer) _result))))
      (else
        (Math|Integer|IncrementInt _enemieskilledarea2
          (:%20%20
            _))))
    (if (and (Variables|/Script/Undertale_HD_2D.MyPlayerCharacter|GetbInArea1 _normalplayer) (== (Variables|/Script/Undertale_HD_2D.MyPlayerCharacter|GetMaxEnemiesArea1 _normalplayer) _result))
      (Variables|/Game/Blueprints/Battles/BP_BattleManager.BP_BattleManager_C|SetCurrentState (Variables|Default|GetBattleManager) "NewEnumerator7")
      (elif (and (== _enemieskilledarea2 (Variables|/Script/Undertale_HD_2D.MyPlayerCharacter|GetMaxEnemiesArea2 _normalplayer_3)) (Variables|/Script/Undertale_HD_2D.MyPlayerCharacter|GetbInArea2 _normalplayer_3))
        (Variables|/Game/Blueprints/Battles/BP_BattleManager.BP_BattleManager_C|SetCurrentState (Variables|Default|GetBattleManager) "NewEnumerator7")))))