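; Battle manager that runs Undertale-style encounters with a randomly picked Rock or Frog enemy, offering Fight, Talk and Mercy.
; A state switch in HandleState drives dialogue, combat, death and exit, reading sprites and lines from the enemy's data asset.
; Timelines scale the battle box between dialogue and fight sizes, toggling widgets and the player's heart.
; The skip input advances dialogue by a counter, then shrinks the box or ends the battle.
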(event Custom|Increase%20Box%20for%20enemy%20death
  (bind _skipwidget (Variables|Default|GetSkipWidget))
  (bind _enemyda (Variables|Default|GetEnemyDA))
  (bind _enemydata (Variables|/Game/Blueprints/Battles/Enemies/DA_EnemyData.DA_EnemyData_C|GetEnemyData _enemyda))
  ;[1 0.8962 0.5284] Increase Box for enemy death
  (Widget|RemovefromParent (Variables|Default|GetHealth%20Wid))
  (Variables|Default|SetDialogue%20count 3)
  (Variables|Default|SetCurrentState "NewEnumerator4")
  (Variables|Default|SetReduced false)
  (bind _enemy (Variables|Default|GetEnemy)
    (:then
      (switch string (.name _enemydata)
        (:Chill%20Rock
          (Rendering|Components|Sprite|SetSprite (Variables|/Game/Blueprints/Battles/Enemies/BP_Enemy.BP_Enemy_C|GetPaperSprite (Variables|Default|GetEnemy)) (Utilities|Array|Get(acopy) (.sprite _enemydata)))
          (bind _scale_lerp (Timeline|Timeline_0 PlayFromStart)
            (:Update
              (Transformation|SetActorScale3D (Variables|Default|GetBattleBox) (Math|Vector|Lerp(Vector) "0.750000,0.750000,1.000000" "1.000000,2.500000,1.000000" _scale_lerp)))
            (:Finished
              (CallFunction|HandleState)
              (UserInterface|Viewport|AddtoViewport (Variables|Default|GetDialogueWidget) 0)
              (UserInterface|Viewport|AddtoViewport _skipwidget 0)
              (Default|FlickerEvent _skipwidget))))
        (:Frog
          (Sprite|SetFlipbook (Variables|/Game/Blueprints/Battles/Enemies/BP_Enemy.BP_Enemy_C|GetPaperFlipbook _enemy))
          (Rendering|Components|Sprite|SetSprite (Variables|/Game/Blueprints/Battles/Enemies/BP_Enemy.BP_Enemy_C|GetPaperSprite (Variables|Default|GetEnemy)) "/Game/Sprite/Enemies/Frog/T_frog_Sprite_2.T_frog_Sprite_2")
          (Timeline|Timeline_0 PlayFromStart))))
    (:else)))

(event Custom|Increaese_box_size
  (bind _skipwidget (Variables|Default|GetSkipWidget))
  (bind _enemyda (Variables|Default|GetEnemyDA))
  (bind _enemydata (Variables|/Game/Blueprints/Battles/Enemies/DA_EnemyData.DA_EnemyData_C|GetEnemyData _enemyda))
  ;[1 0.7562 0.5386] INCREASE BOX
  (Widget|RemovefromParent (Variables|Default|GetHealth%20Wid))
  (Variables|Default|SetReduced false)
  (bind _enemy (Variables|Default|GetEnemy)
    (:then
      (switch string (.name _enemydata)
        (:Chill%20Rock
          (Rendering|Components|Sprite|SetSprite (Variables|/Game/Blueprints/Battles/Enemies/BP_Enemy.BP_Enemy_C|GetPaperSprite (Variables|Default|GetEnemy)) (Utilities|Array|Get(acopy) (.sprite _enemydata)))
          (bind _scale_lerp (Timeline|increase%20box%20size PlayFromStart)
            (:Update
              (Transformation|SetActorScale3D (Variables|Default|GetBattleBox) (Math|Vector|Lerp(Vector) "0.750000,0.750000,1.000000" "1.000000,2.500000,1.000000" _scale_lerp)))
            (:Finished
              (UserInterface|Viewport|AddtoViewport (Variables|Default|GetDialogueWidget) 0)
              (UserInterface|Viewport|AddtoViewport _skipwidget 0)
              (Default|FlickerEvent _skipwidget))))
        (:Frog
          (Sprite|SetFlipbook (Variables|/Game/Blueprints/Battles/Enemies/BP_Enemy.BP_Enemy_C|GetPaperFlipbook _enemy) (.paperflipbook _enemydata))
          (Rendering|Components|Sprite|SetSprite (Variables|/Game/Blueprints/Battles/Enemies/BP_Enemy.BP_Enemy_C|GetPaperSprite (Variables|Default|GetEnemy)) 0)
          (Timeline|increase%20box%20size PlayFromStart))))
    (:else)))

(event Custom|Update%20Health%20UI
  (params (Current%20HP :type Integer) (Max%20HP :type Integer))
  (bind _health_wid (Variables|Default|GetHealth%20Wid))
  ;[1 1 1] Update Health HP
  (Variables|/Game/UI/Combat/WB_PlayerHealth.WB_PlayerHealth_C|SetCurrent%20HP _health_wid (Utilities|Text|ToText(Integer) Current%20HP))
  (Variables|/Game/UI/Combat/WB_PlayerHealth.WB_PlayerHealth_C|SetMAX%20Health _health_wid (Utilities|Text|ToText(Integer) Max%20HP)))

(event Custom|Reduce_box_size
  (bind _normalplayer (Variables|Default|GetNormalPlayer))
  (bind _mercybutton (Variables|Default|GetMercyButton))
  ;[0.4579 1 0.9801] REDUCE BOX
  (if (not (Variables|Default|GetReduced))
    (Widget|RemovefromParent (Variables|Default|GetDialogueWidget))
    (bind _scale_lerp (Timeline|Timeline PlayFromStart)
      (:Update
        (Transformation|SetActorScale3D (Variables|Default|GetBattleBox) (Math|Vector|Lerp(Vector) "1.000000,2.500000,1.000000" "0.750000,0.750000,1.000000" _scale_lerp)))
      (:Finished
        (UserInterface|Viewport|AddtoViewport (Variables|Default|GetHealth%20Wid) 0)
        (if (Variables|Default|GetSpawned)
          _
          (else
            (Class|MyPlayerCharacter|SpawnHeart _normalplayer)
            (Variables|Default|SetSpawned true)))
        (Class|MyPlayerCharacter|ShowHeart _normalplayer)
        (Variables|Default|SetReduced true)
        (if (Variables|Default|GetFigthed)
          (Widget|RemovefromParent (Variables|Default|GetTalkButton))
          (UserInterface|Viewport|AddtoViewport (Variables|Default|GetNot%20active%20talk) 0)
          (Default|InteractableFight (Variables|Default|GetFightButton))
          (else
            (Default|InteractableFight (Variables|Default|GetFightButton))
            (if (Variables|Default|GetTalked)
              (Widget|RemovefromParent (Variables|Default|GetTalkButton))
              (UserInterface|Viewport|AddtoViewport (Variables|Default|GetNot%20active%20talk) 0)
              (if (Variables|Default|GetActiveMercy)
                (Widget|RemovefromParent (Variables|Default|GetNotActiveMercy))
                (Default|InteractableMercy _mercybutton)
                (UserInterface|Viewport|AddtoViewport _mercybutton 0))
              (else
                (Default|InteractableTalk (Variables|Default|GetTalkButton))))))))))

(event Custom|Activate%20Dialogue
  ;[0.9962 0.3889 1] Activate Talk Dialogue
  (Variables|Default|SetTalked true)
  (CallFunction|IncreaseBoxforTalk))

(event Custom|Increase%20Box%20for%20Talk
  (bind _enemyda (Variables|Default|GetEnemyDA))
  (bind _enemydata (Variables|/Game/Blueprints/Battles/Enemies/DA_EnemyData.DA_EnemyData_C|GetEnemyData _enemyda))
  ;[1 0.6381 0.5276] Increase Box for Talk button
  (Widget|RemovefromParent (Variables|Default|GetHealth%20Wid))
  (Class|MyPlayerCharacter|HideHeart (Variables|Default|GetNormalPlayer))
  (Variables|Default|SetReduced false)
  (bind _enemy (Variables|Default|GetEnemy)
    (:then
      (switch string (.name _enemydata)
        (:Chill%20Rock
          (Rendering|Components|Sprite|SetSprite (Variables|/Game/Blueprints/Battles/Enemies/BP_Enemy.BP_Enemy_C|GetPaperSprite (Variables|Default|GetEnemy)) (Utilities|Array|Get(acopy) (.sprite _enemydata)))
          (bind _scale_lerp (Timeline|Timeline_1 PlayFromStart)
            (:Update
              (Transformation|SetActorScale3D (Variables|Default|GetBattleBox) (Math|Vector|Lerp(Vector) "0.750000,0.750000,1.000000" "1.000000,2.500000,1.000000" _scale_lerp)))
            (:Finished
              (Variables|Default|SetCurrentState "NewEnumerator6")
              (CallFunction|HandleState))))
        (:Frog
          (Sprite|SetFlipbook (Variables|/Game/Blueprints/Battles/Enemies/BP_Enemy.BP_Enemy_C|GetPaperFlipbook _enemy) (.paperflipbook _enemydata))
          (Rendering|Components|Sprite|SetSprite (Variables|/Game/Blueprints/Battles/Enemies/BP_Enemy.BP_Enemy_C|GetPaperSprite (Variables|Default|GetEnemy)) 0)
          (Timeline|Timeline_1 PlayFromStart))))
    (:else)))

(event Custom|Mercy%20Dialogue
  (bind _dialoguewidget (Variables|Default|GetDialogueWidget))
  (bind _skipwidget (Variables|Default|GetSkipWidget))
  ;[0.4033 0.5455 1] Mercy or no mercy dialogue
  (Variables|Default|SetActiveMercy true)
  (Variables|Default|SetDialogue%20index 0)
  (UserInterface|Viewport|AddtoViewport _skipwidget 0)
  (Default|FlickerEvent _skipwidget)
  (UserInterface|Viewport|AddtoViewport _dialoguewidget 0)
  (Default|UpdateDialogue _dialoguewidget (Utilities|Array|Get(acopy) (.dialogueresponsemercy (Variables|/Game/Blueprints/Battles/Enemies/DA_EnemyData.DA_EnemyData_C|GetEnemyData (Variables|Default|GetEnemyDA))) (Variables|Default|GetDialogue%20index)))
  (Variables|Default|SetXActive true))

(event Custom|No%20mercy%20Dialogue
  (bind _skipwidget (Variables|Default|GetSkipWidget))
  (bind _dialoguewidget (Variables|Default|GetDialogueWidget))
  ;[0.4033 0.5455 1] Mercy or no mercy dialogue
  (Variables|Default|SetDialogue%20index 0)
  (UserInterface|Viewport|AddtoViewport _skipwidget 0)
  (Default|FlickerEvent _skipwidget)
  (UserInterface|Viewport|AddtoViewport _dialoguewidget 0)
  (Default|UpdateDialogue _dialoguewidget (Utilities|Array|Get(acopy) (.dialogueresponsenomercy (Variables|/Game/Blueprints/Battles/Enemies/DA_EnemyData.DA_EnemyData_C|GetEnemyData (Variables|Default|GetEnemyDA))) (Variables|Default|GetDialogue%20index)))
  (Variables|Default|SetXActive true))

(event Custom|Pressed%20Mercy
  (bind _skipwidget (Variables|Default|GetSkipWidget))
  (bind _dialoguewidget (Variables|Default|GetDialogueWidget))
  ;[0.4444 1 0.4482] Mercied
  (Widget|RemovefromParent (Variables|Default|GetHealth%20Wid))
  (Input|SetInputModeGameOnly (Game|GetPlayerController 0) false)
  (Variables|Default|SetReduced false)
  (Variables|Default|SetMercied true)
  (Class|MyPlayerCharacter|HideHeart (Variables|Default|GetNormalPlayer))
  (bind _scale_lerp (Timeline|Timeline_2 PlayFromStart)
    (:Update
      (Transformation|SetActorScale3D (Variables|Default|GetBattleBox) (Math|Vector|Lerp(Vector) "0.750000,0.750000,1.000000" "1.000000,2.500000,1.000000" _scale_lerp)))
    (:Finished
      (UserInterface|Viewport|AddtoViewport _skipwidget 0)
      (Default|FlickerEvent _skipwidget)
      (Variables|Default|SetDialogue%20index 0)
      (Variables|Default|SetDialogue%20count 4)
      (UserInterface|Viewport|AddtoViewport _dialoguewidget 0)
      (Default|UpdateDialogue _dialoguewidget (Utilities|Array|Get(acopy) (.mercydialague (Variables|/Game/Blueprints/Battles/Enemies/DA_EnemyData.DA_EnemyData_C|GetEnemyData (Variables|Default|GetEnemyDA))) (Variables|Default|GetDialogue%20index)))
      (Variables|Default|SetXActive true))))

(event Custom|Increase%20for%20no%20enemy%20left
  (bind _skipwidget (Variables|Default|GetSkipWidget))
  ;[1 0.4079 0.3281] Increase box for no enemy in area
  (Class|MyPlayerCharacter|HideHeart (Variables|Default|GetNormalPlayer))
  (Variables|Default|SetReduced false)
  (bind _scale_lerp (Timeline|Timeline_3 PlayFromStart)
    (:Update
      (Transformation|SetActorScale3D (Variables|Default|GetBattleBox) (Math|Vector|Lerp(Vector) "0.750000,0.750000,1.000000" "1.000000,2.500000,1.000000" _scale_lerp)))
    (:Finished
      (Variables|Default|SetDialogue%20index 0)
      (Variables|Default|SetDialogue%20count 5)
      (Default|UpdateDialogue (Variables|Default|GetDialogueWidget) (Utilities|Array|Get(acopy) (Variables|Default|GetNoEnemyText)))
      (UserInterface|Viewport|AddtoViewport (Variables|Default|GetDialogueWidget) 0)
      (Default|FlickerEvent _skipwidget)
      (UserInterface|Viewport|AddtoViewport _skipwidget 0)
      (Variables|Default|SetXActive true))))

(event Input|EnhancedActionEvents|EnhancedInputActionIA_SkipDialogue
  (params (ActionValue :type Boolean) (ElapsedSeconds :type Float%20%28double-precision%29) (TriggeredSeconds :type Float%20%28double-precision%29) (InputAction :type Input%20Action%20Object%20Reference :default "/Game/Inputs/IA_SkipDialogue.IA_SkipDialogue"))
  ;[1 0.4272 0.1094] SKIP DIALOGUE
  (:Started
    (if (Variables|Default|GetXActive)
      (switch int (Variables|Default|GetDialogue%20count)
        (:1
          (CallFunction|SkipDialogue (.firstdialogue (Variables|/Game/Blueprints/Battles/Enemies/DA_EnemyData.DA_EnemyData_C|GetEnemyData (Variables|Default|GetEnemyDA)))))
        (:2
          (CallFunction|SkipDialogue (.2nddialogue (Variables|/Game/Blueprints/Battles/Enemies/DA_EnemyData.DA_EnemyData_C|GetEnemyData (Variables|Default|GetEnemyDA)))))
        (:3
          (CallFunction|SkipDialogue (.deathdialogue (Variables|/Game/Blueprints/Battles/Enemies/DA_EnemyData.DA_EnemyData_C|GetEnemyData (Variables|Default|GetEnemyDA)))))
        (:4
          (CallFunction|SkipDialogue (.mercydialague (Variables|/Game/Blueprints/Battles/Enemies/DA_EnemyData.DA_EnemyData_C|GetEnemyData (Variables|Default|GetEnemyDA)))))
        (:5
          (Default|Pressed (Variables|Default|GetSkipWidget))
          (Utilities|FlowControl|Delay 0.5)
          (Widget|RemovefromParent (Variables|Default|GetDialogueWidget))
          (Class|MyPlayerCharacter|ExitCombat (Variables|Default|GetNormalPlayer))
          (Variables|Default|SetXActive false))))))

(event EventBeginPlay
  ;[1 1 1] BEGIN SETUP
  (bind _returnvalue (UserInterface|CreateWidget "/Game/UI/Combat/Dialogue/WB_InteractableDialogue.WB_InteractableDialogue_C"))
  (Variables|Default|SetInteractableDialogue _returnvalue)
  (bind _returnvalue_2 (UserInterface|CreateWidget "/Game/UI/Combat/Dialogue/WB_NormalDialogue.WB_NormalDialogue_C"))
  (Variables|Default|SetDialogueWidget _returnvalue_2)
  (bind _returnvalue_3 (UserInterface|CreateWidget "/Game/UI/Combat/Dialogue/WB_TriangleDialogue.WB_TriangleDialogue_C"))
  (Variables|Default|SetSkipWidget _returnvalue_3)
  (bind _returnvalue_4 (UserInterface|CreateWidget "/Game/UI/Combat/WB_TalkButton.WB_TalkButton_C"))
  (Variables|Default|SetTalkButton _returnvalue_4)
  (bind _returnvalue_5 (UserInterface|CreateWidget "/Game/UI/Combat/WB_FightButton.WB_FightButton_C"))
  (Variables|Default|SetFightButton _returnvalue_5)
  (bind _returnvalue_6 (UserInterface|CreateWidget "/Game/UI/Combat/WB_MercyButton.WB_MercyButton_C"))
  (Variables|Default|SetMercyButton _returnvalue_6)
  (bind _returnvalue_7 (UserInterface|CreateWidget "/Game/UI/Combat/WB_MercyNotActive.WB_MercyNotActive_C"))
  (Variables|Default|SetNotActiveMercy _returnvalue_7)
  (bind _returnvalue_8 (UserInterface|CreateWidget "/Game/UI/Combat/WB_TalkNotActive.WB_TalkNotActive_C"))
  (Variables|Default|SetNot%20active%20talk _returnvalue_8)
  (bind _returnvalue_9 (UserInterface|CreateWidget "/Game/UI/Combat/WB_FightNotActive.WB_FightNotActive_C"))
  (Variables|Default|SetNot%20Active%20Fight _returnvalue_9)
  (Input|EnableInput (Game|GetPlayerController 0))
  (bind _outactors (Actor|GetAllActorsOfClasswithTag "/Game/Blueprints/MainCharacter/NormalPlayer/BP_PlayerCharacter.BP_PlayerCharacter_C" "Player Character"))
  (Variables|Default|SetNormalPlayer (Utilities|Array|Get(acopy) _outactors))
  (bind _returnvalue_10 (UserInterface|CreateWidget "/Game/UI/Combat/WB_PlayerHealth.WB_PlayerHealth_C"))
  (Variables|Default|SetHealth%20Wid _returnvalue_10))

(event EventChangeHealth
  (params (Current%20Health :type Integer) (Max%20Health :type Integer)))

(fn ConstructionScript)

(fn HandleState
  (switch Utilities|FlowControl|Switch|SwitchonE_BattleEvent (Variables|Default|GetCurrentState)
    (:NewEnumerator0
      (switch int (Math|Integer|%(Integer) (Math|Random|RandomIntegerinRange 1 20) 2)
        (:0
          (Variables|Default|SetEnemyDA "/Game/Blueprints/Battles/Enemies/DA_Rock.DA_Rock"))
        (:1
          (Variables|Default|SetEnemyDA "/Game/Blueprints/Battles/Enemies/DA_Frog.DA_Frog")))
      (CallFunction|StartFirstDialogue))
    (:NewEnumerator1
      (CallFunction|StartBattle))
    (:NewEnumerator2
      (CallFunction|StartSecondDialogue))
    (:NewEnumerator3
      (CallFunction|EndBattle))
    (:NewEnumerator4
      (CallFunction|EnemyDeathScene))
    (:NewEnumerator6
      (CallFunction|DialogueInteractions))
    (:NewEnumerator7
      (CallFunction|DisplayNoEnemy))))

(fn StartFirstDialogue
  (Variables|Default|SetMercied false)
  (Variables|Default|SetExiting%20for%20death false)
  (Variables|Default|SetActiveMercy false)
  (Variables|Default|SetTalked false)
  (Variables|Default|SetFigthed false)
  (Variables|Default|SetSprite%20color (Variables|/Script/Paper2D.PaperSpriteComponent|GetSpriteColor (Variables|/Game/Blueprints/Battles/Enemies/BP_Enemy.BP_Enemy_C|GetPaperSprite (Variables|Default|GetEnemy))))
  (UserInterface|Viewport|AddtoViewport (Variables|Default|GetFightButton) 0)
  (UserInterface|Viewport|AddtoViewport (Variables|Default|GetTalkButton) 0)
  (UserInterface|Viewport|AddtoViewport (Variables|Default|GetNotActiveMercy) 0)
  (CallFunction|IncreaeseBoxSize)
  (Variables|Default|SetDialogue%20index 0)
  (Default|UpdateDialogue (Variables|Default|GetDialogueWidget) (Utilities|Array|Get(acopy) (.firstdialogue (Variables|/Game/Blueprints/Battles/Enemies/DA_EnemyData.DA_EnemyData_C|GetEnemyData (Variables|Default|GetEnemyDA))) (Variables|Default|GetDialogue%20index)))
  (Variables|Default|SetXActive true))

(fn StartBattle
  (bind _normalplayer (Variables|Default|GetNormalPlayer))
  (Variables|Default|SetFigthed true)
  (Input|SetInputModeGameOnly (Game|GetPlayerController 0) false)
  (Variables|Default|SetXActive false)
  (if (Variables|Default|GetReduced)
    _
    (else
      (CallFunction|ReduceBoxSize)
      (Variables|Default|SetReduced true)))
  (if (Variables|Default|GetSpawned)
    _
    (else
      (Class|MyPlayerCharacter|SpawnHeart _normalplayer)
      (Variables|Default|SetSpawned true)))
  (Class|MyPlayerCharacter|ShowHeart _normalplayer)
  (Default|StartFight (Variables|Default|GetEnemy) (.name (Variables|/Game/Blueprints/Battles/Enemies/DA_EnemyData.DA_EnemyData_C|GetEnemyData (Variables|Default|GetEnemyDA)))))

(fn RemoveDialogue
  (Widget|RemovefromParent (Variables|Default|GetDialogueWidget)))

(fn EndBattle
  (bind _enemy (Variables|Default|GetEnemy))
  (Variables|Default|SetXActive false)
  (Variables|Default|SetSpawned false)
  (Variables|Default|SetDialogue%20index 0)
  (Variables|Default|SetDialogue%20count 1)
  (Variables|Default|SetCurrentState "NewEnumerator0")
  (Input|SetInputModeGameOnly (Game|GetPlayerController 0) false)
  (Sprite|SetFlipbook (Variables|/Game/Blueprints/Battles/Enemies/BP_Enemy.BP_Enemy_C|GetPaperFlipbook _enemy))
  (Rendering|Components|Sprite|SetSprite (Variables|/Game/Blueprints/Battles/Enemies/BP_Enemy.BP_Enemy_C|GetPaperSprite _enemy) 0)
  (Widget|RemovefromParent (Variables|Default|GetFightButton))
  (Class|MyPlayerCharacter|ExitCombat (Variables|Default|GetNormalPlayer))
  (Default|CheckforNoEnemy (Variables|Default|GetEnemy)))

(fn SkipDialogue
  (params (Dialogue%20Array :type Array%20of%20Texts))
  (Variables|Default|SetDialogue%20index (+ 1 (Variables|Default|GetDialogue%20index)))
  (if (== (Utilities|Array|Length Dialogue%20Array) (Variables|Default|GetDialogue%20index))
    (Widget|RemovefromParent (Variables|Default|GetSkipWidget))
    (if (Variables|Default|GetTalked)
      _
      (else
        (Math|Integer|IncrementInt (Variables|Default|GetDialogue%20count)
          (:%20%20
            _))))
    (if (or (Variables|Default|GetExiting%20for%20death) (Variables|Default|GetMercied))
      (Widget|RemovefromParent (Variables|Default|GetDialogueWidget))
      (Variables|Default|SetCurrentState "NewEnumerator3")
      (CallFunction|HandleState)
      (else
        (CallFunction|ReduceBoxSize)))
    (else
      (Default|UpdateDialogue (Variables|Default|GetDialogueWidget) (Utilities|Array|Get(acopy) Dialogue%20Array (Variables|Default|GetDialogue%20index)))
      (Default|Pressed (Variables|Default|GetSkipWidget)))))

(fn UnfocusWidget
  (Input|SetInputModeGameOnly (Game|GetPlayerController 0) false))

(fn StartSecondDialogue
  (Class|MyPlayerCharacter|HideHeart (Variables|Default|GetNormalPlayer))
  (CallFunction|IncreaeseBoxSize)
  (Variables|Default|SetDialogue%20index 0)
  (Default|UpdateDialogue (Variables|Default|GetDialogueWidget) (Utilities|Array|Get(acopy) (.2nddialogue (Variables|/Game/Blueprints/Battles/Enemies/DA_EnemyData.DA_EnemyData_C|GetEnemyData (Variables|Default|GetEnemyDA))) (Variables|Default|GetDialogue%20index)))
  (Variables|Default|SetXActive true))

(fn EnemyDeathScene
  (Variables|Default|SetExiting%20for%20death true)
  (Variables|Default|SetDialogue%20index 0)
  (Default|UpdateDialogue (Variables|Default|GetDialogueWidget) (Utilities|Array|Get(acopy) (.deathdialogue (Variables|/Game/Blueprints/Battles/Enemies/DA_EnemyData.DA_EnemyData_C|GetEnemyData (Variables|Default|GetEnemyDA))) (Variables|Default|GetDialogue%20index)))
  (Variables|Default|SetXActive true))

(fn DialogueInteractions
  (bind _interactabledialogue (Variables|Default|GetInteractableDialogue))
  (UserInterface|Viewport|AddtoViewport _interactabledialogue 0)
  (Widget|SetFocus _interactabledialogue)
  (Default|PopulateOptions _interactabledialogue (.dialogueoptions (Variables|/Game/Blueprints/Battles/Enemies/DA_EnemyData.DA_EnemyData_C|GetEnemyData (Variables|Default|GetEnemyDA)))))

(fn DisplayNoEnemy
  (Variables|Default|SetMercied false)
  (Variables|Default|SetExiting%20for%20death false)
  (Variables|Default|SetActiveMercy false)
  (Variables|Default|SetTalked false)
  (Variables|Default|SetFigthed false)
  (UserInterface|Viewport|AddtoViewport (Variables|Default|GetNot%20Active%20Fight) 0)
  (UserInterface|Viewport|AddtoViewport (Variables|Default|GetNot%20active%20talk) 0)
  (UserInterface|Viewport|AddtoViewport (Variables|Default|GetNotActiveMercy) 0)
  (Variables|Default|SetEnemyDA 0)
  (CallFunction|IncreaseforNoEnemyLeft))