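; Dialogue component for the old turtle NPC, who points the player toward their lost dog and explains the FIGHT, TALK and MERCY combat options.
; It extends a parent Dialogue function, switching on DialogueTreeIndex to add lines, show a reply option and branch on it.
; It calls SwitchCamera on the owning BP_NPCTurtle at key beats.
; Closing sets the index back to the tutorial lines and flags the dialogue finished.
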(event EventBeginPlay)

(event EventTick
  (params (DeltaSeconds :type Float%20%28single-precision%29)))

(fn Dialogue
  (|CallParentFunction)
  (switch int (Variables|Default|GetDialogue%20Tree%20Index)
    (:1
      (CallFunction|AddDialogue "An old Turtle" "Wait! Stay right there! 
 
**cough cough press x to let me talk further cough cough**")
      (bind _asbp_npcturtle (Utilities|Casting|CastToBP_NPCTurtle (Components|GetOwner)))
      (bind _output_get (Variables|Default|SetOwner _asbp_npcturtle))
      (Default|SwitchCamera _output_get))
    (:2
      (CallFunction|AddDialogue "An old Turtle" "Who are you? I hardly see humans down here."))
    (:3
      (Variables|Default|SetX%20active false)
      (CallFunction|ShowOptions (Utilities|Array|MakeArray "I'm just looking for a dog, have you seen him?")))
    (:4
      (Variables|Default|SetProgress false)
      (Variables|Default|SetX%20active true)
      (switch int (Variables|Default|GetDialogue%20Index)
        (:0
          (bind _d_state (CallFunction|AddDialogue "An old Turtle" "A dog?" 0 1))
          (switch Utilities|FlowControl|Switch|SwitchonE_NPCDialogueState _d_state
            (:NewEnumerator0
              (CallFunction|AddDialogue "An old Turtle" "Ah yes, I think I saw one running deeper into the cave. Maybe you can try looking for it in the village " 0 2)
              (Variables|Default|SetDialogue%20Tree%20Index 5)
              (Variables|Default|SetProgress true)
              (Default|SwitchCamera (Variables|Default|GetOwner)))))))
    (:6
      (CallFunction|AddDialogue "An old Turtle" "Oh. And child... Our kind is often untrusting of humans.")
      (Default|SwitchCamera (Variables|Default|GetOwner)))
    (:7
      (CallFunction|AddDialogue "An old Turtle" "If somebody attacks you please don't hurt them by pressing FIGHT and timing your attack by pressing SPACEBAR."))
    (:8
      (CallFunction|AddDialogue "An old Turtle" "You can just TALK to them. If they like you, you could just have MERCY."))
    (:9
      (CallFunction|AddDialogue "An old Turtle" "Good luck finding your dog."))
    (:10
      (CallFunction|CloseConversation)
      (Variables|Default|SetDialogue%20Tree%20Index 6)
      (Variables|Default|SetFinished%20Dialogue true))))