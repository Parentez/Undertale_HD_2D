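; NPC actor with an animated E-key interaction prompt and a three-shot camera sequence, presumably for player interactions.
; Each SwitchCamera call increments a counter that is never reset here, activates the next camera and makes the NPC the view target.
; Per-shot timelines then lerp that camera toward its paired camera component, which serves as an end-pose marker.
; Construction caches the PlayerPosition transform and the prompt's start location, from which the key animates upward.
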(event Custom|Blend%20Camera%203
  (params (Camera%20position%20input :type Vector) (Camera%20Rotation%20input :type Rotator) (Camera%20Position%20Output :type Vector) (Camera%20Rotation%20output :type Rotator) (Camera%20to%20lerp :type Camera%20Component%20Object%20Reference))
  ;[1 1 1] Blend Camera views
  (bind _lerp_camera_position (Timeline|Timeline_0 Play)
    (:Update
      (Transformation|SetRelativeLocationAndRotation Camera%20to%20lerp (Math|Vector|Lerp(Vector) Camera%20position%20input Camera%20Position%20Output _lerp_camera_position) (Math|Rotator|Lerp(Rotator) Camera%20Rotation%20input Camera%20Rotation%20output _lerp_camera_position) false false))))

(event Custom|Blend%20Camera%201
  (params (Camera%20position%20input :type Vector) (Camera%20Rotation%20input :type Rotator) (Camera%20Position%20Output :type Vector) (Camera%20Rotation%20output :type Rotator) (Camera%20to%20lerp :type Camera%20Component%20Object%20Reference))
  ;[1 1 1] Blend Camera views
  (bind _lerp_camera_position (Timeline|Camera%20blen Play)
    (:Update
      (Transformation|SetRelativeLocationAndRotation Camera%20to%20lerp (Math|Vector|Lerp(Vector) Camera%20position%20input Camera%20Position%20Output _lerp_camera_position) (Math|Rotator|Lerp(Rotator) Camera%20Rotation%20input Camera%20Rotation%20output _lerp_camera_position) false false))))

(event Custom|Show%20E%20key
  (bind _start_ekey_location (Variables|Default|GetStart%20Ekey%20location))
  (bind _lerp (Timeline|E%20key%20Anim PlayFromStart)
    (:Update
      (Transformation|SetRelativeLocation (Variables|Default|GetE%20key) (Math|Vector|Lerp(Vector) (Variables|Default|GetStart%20Ekey%20location) (Math|Vector|MakeVector (.x _start_ekey_location) (.y _start_ekey_location) (+ (.z _start_ekey_location) 15.0)) _lerp) false false))))

(event Custom|Blend%20Camera%202
  (params (Camera%20position%20input :type Vector) (Camera%20Rotation%20input :type Rotator) (Camera%20Position%20Output :type Vector) (Camera%20Rotation%20output :type Rotator) (Camera%20to%20lerp :type Camera%20Component%20Object%20Reference))
  ;[1 1 1] Blend Camera views
  (bind _lerp_camera_position (Timeline|Timeline Play)
    (:Update
      (Transformation|SetRelativeLocationAndRotation Camera%20to%20lerp (Math|Vector|Lerp(Vector) Camera%20position%20input Camera%20Position%20Output _lerp_camera_position) (Math|Rotator|Lerp(Rotator) Camera%20Rotation%20input Camera%20Rotation%20output _lerp_camera_position) false false))))

(event Custom|E%20key%20visible
  (Rendering|SetVisibility (Variables|Default|GetE%20key) true false)
  (Development|PrintText "E key")
  (CallFunction|ShowEKey))

(event Custom|Hide%20E%20key
  (Rendering|SetVisibility (Variables|Default|GetE%20key) false false))

(event EventSetInteractableState
  (params (Show%20Interact :type Boolean))
  (if Show%20Interact
    (Development|PrintText (Variables|Default|GetNpcName))))

(fn ConstructionScript
  (bind _player_position (Variables|Default|GetPlayer%20Position))
  (Variables|Default|SetPlayerPosition (Transformation|GetWorldLocation _player_position))
  (Variables|Default|SetPlayerRotation (Transformation|GetWorldRotation _player_position))
  (Variables|Default|SetStart%20Ekey%20location (Variables|/Script/Engine.SceneComponent|GetRelativeLocation (Variables|Default|GetE%20key))))

(fn SwitchCamera
  (bind _camera3 (Variables|Default|GetCamera3))
  (bind _camera2 (Variables|Default|GetCamera2))
  (bind _camera1_1 (Variables|Default|GetCamera1_1))
  (bind _camera1 (Variables|Default|GetCamera1))
  (bind _camera3_3 (Variables|Default|GetCamera3_3))
  (bind _camera2_2 (Variables|Default|GetCamera2_2))
  (bind _camera2_2 (Variables|Default|GetCamera2))
  (bind _camera3_2 (Variables|Default|GetCamera3))
  (bind _camera1_2 (Variables|Default|GetCamera1))
  (Math|Integer|IncrementInt (Variables|Default|GetCamera%20switch)
    (:%20%20
      (switch int (Variables|Default|GetCamera%20switch)
        (:1
          (Development|PrintText "camera 1")
          (Components|Activation|SetActive (Variables|Default|GetCamera2) false false)
          (Components|Activation|SetActive _camera1_2 true false)
          (Game|Player|SetViewTargetwithBlend (Game|GetPlayerController 0) (Components|GetOwner _camera1_2) 0.0 "VTBlend_Linear" 0.0 false)
          (CallFunction|BlendCamera1 (Variables|/Script/Engine.SceneComponent|GetRelativeLocation _camera1) (Variables|/Script/Engine.SceneComponent|GetRelativeRotation _camera1) (Variables|/Script/Engine.SceneComponent|GetRelativeLocation _camera1_1) (Variables|/Script/Engine.SceneComponent|GetRelativeRotation _camera1_1) _camera1_2))
        (:2
          (Development|PrintText "camera 2")
          (Components|Activation|SetActive (Variables|Default|GetCamera3) false false)
          (Components|Activation|SetActive _camera2 true false)
          (Game|Player|SetViewTargetwithBlend (Game|GetPlayerController 0) (Components|GetOwner _camera2) 0.0 "VTBlend_Linear" 0.0 false)
          (CallFunction|BlendCamera2 (Variables|/Script/Engine.SceneComponent|GetRelativeLocation _camera2_2) (Variables|/Script/Engine.SceneComponent|GetRelativeRotation _camera2_2) (Variables|/Script/Engine.SceneComponent|GetRelativeLocation _camera2_2) (Variables|/Script/Engine.SceneComponent|GetRelativeRotation _camera2_2) _camera2_2))
        (:3
          (Development|PrintText "camera 3")
          (Components|Activation|SetActive (Variables|Default|GetCamera1) false false)
          (Components|Activation|SetActive _camera3 true false)
          (Game|Player|SetViewTargetwithBlend (Game|GetPlayerController 0) (Components|GetOwner _camera3) 0.0 "VTBlend_Linear" 0.0 false)
          (CallFunction|BlendCamera3 (Variables|/Script/Engine.SceneComponent|GetRelativeLocation _camera3_2) (Variables|/Script/Engine.SceneComponent|GetRelativeRotation _camera3_2) (Variables|/Script/Engine.SceneComponent|GetRelativeLocation _camera3_3) (Variables|/Script/Engine.SceneComponent|GetRelativeRotation _camera3_3) _camera3_2))))))