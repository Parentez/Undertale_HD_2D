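; BP_NPCLizard is an interactable lizard NPC that runs a conversation through its ACNpcLizard component.
; Interacting hides the E-key prompt, enables input, stores the instigator and opens the conversation, then sets the component's XActive flag after a one-second delay.
; The skip-dialogue event advances the dialogue only while XActive is set, so skipping is blocked during that first second.
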(event EventInteract
  (params (Instigator :type Actor%20Object%20Reference))
  (CallFunction|HideEKey)
  (Variables|Default|SetActivate%20Input true)
  (Variables|Default|SetInteract%20Instigator Instigator)
  (Default|OpenConversation (Variables|Default|GetAC_NpcLizard))
  (Utilities|FlowControl|Delay 1.0)
  (Variables|/Game/Blueprints/NPC/AC_NpcDialogue.AC_NpcDialogue_C|SetX%20active (Variables|Default|GetAC_NpcLizard) true))

(event EventSkipDialogue
  (if (Variables|/Game/Blueprints/NPC/AC_NpcDialogue.AC_NpcDialogue_C|GetX%20active (Variables|Default|GetAC_NpcLizard))
    (Default|ProgressDialogue (Variables|Default|GetAC_NpcLizard))))

(fn ConstructionScript
  (|CallParentFunction))