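; Dialogue component for the Jane Frog NPC, who worries about her husband and reacts to the player's choice of four replies about him.
; An override of the parent Dialogue function steps through a DialogueTreeIndex switch, branching on DialogueIndex for the chosen reply.
; Once the talk ends, the saved choice selects a short repeat line for later visits.
; It also toggles the owning BP_NPCFrog's camera at conversation beats.
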(event EventBeginPlay)

(event EventTick
  (params (DeltaSeconds :type Float%20%28single-precision%29)))

(fn Dialogue
  (|CallParentFunction)
  (switch int (Variables|Default|GetDialogue%20Tree%20Index)
    (:1
      (CallFunction|AddDialogue "JANE FROG" "Hello child.")
      (bind _asbp_npcfrog (Utilities|Casting|CastToBP_NPCFrog (Components|GetOwner)))
      (bind _output_get (Variables|Default|Setowner _asbp_npcfrog))
      (Default|SwitchCamera _output_get))
    (:2
      (CallFunction|AddDialogue "JANE FROG" "My husband went grocery shopping to feed our children. I hope he's doing well."))
    (:3
      (Variables|Default|SetX%20active false)
      (CallFunction|ShowOptions (Utilities|Array|MakeArray "Oh yes i found him, he's doing fine" "Never seen him" "CRA!" "I killed him")))
    (:4
      (Default|SwitchCamera (Variables|Default|Getowner))
      (Variables|Default|SetProgress false)
      (Variables|Default|SetX%20active true)
      (switch int (Variables|Default|GetDialogue%20Index)
        (:0
          (bind _d_state (CallFunction|AddDialogue "JANE FROG" "Really?! I hope he returns soon then." 0 1))
          (switch Utilities|FlowControl|Switch|SwitchonE_NPCDialogueState _d_state
            (:NewEnumerator0
              (CallFunction|AddDialogue "JANE FROG" "Thank you though at least I know he's alrigth." 0 2)
              (Variables|Default|SetDialogue%20Tree%20Index 5))))
        (:1
          (bind _d_state_2 (CallFunction|AddDialogue "JANE FROG" "Oh well nevermind." 0 1))
          (switch Utilities|FlowControl|Switch|SwitchonE_NPCDialogueState _d_state_2
            (:NewEnumerator0
              (CallFunction|AddDialogue "JANE FROG" "See you. Craaa" 0 2)
              (Variables|Default|SetDialogue%20Tree%20Index 5))))
        (:2
          (bind _d_state_3 (CallFunction|AddDialogue "JANE FROG" "Oh right I forgot, CRA CRA!" 0 1))
          (switch Utilities|FlowControl|Switch|SwitchonE_NPCDialogueState _d_state_3
            (:NewEnumerator0
              (CallFunction|AddDialogue "JANE FROG" "CRAAAAZY" 0 2)
              (Variables|Default|SetDialogue%20Tree%20Index 5))))
        (:3
          (bind _d_state_4 (CallFunction|AddDialogue "JANE FROG" "WHHHHAAAAAATTTTT????????" 0 1))
          (switch Utilities|FlowControl|Switch|SwitchonE_NPCDialogueState _d_state_4
            (:NewEnumerator0
              (CallFunction|AddDialogue "JANE FROG" "I will never forgive you, what should  i tell to my kids????" 0 2)
              (Variables|Default|SetDialogue%20Tree%20Index 5)))))
      (Default|SwitchCamera (Variables|Default|Getowner))
      (Variables|Default|SetFinished%20Dialogue true))
    (:5
      (switch int (Variables|Default|GetDialogue%20Index)
        (:0
          (Variables|Default|SetDialogue%20Tree%20Index 6))
        (:1
          (Variables|Default|SetDialogue%20Tree%20Index 7))
        (:2
          (Variables|Default|SetDialogue%20Tree%20Index 8))
        (:3
          (Variables|Default|SetDialogue%20Tree%20Index 9)))
      (Variables|/Game/Blueprints/NPC/BP_NPC.BP_NPC_C|SetCamera%20switch (Variables|Default|Getowner) 2)
      (CallFunction|CloseConversation))
    (:6
      (Default|SwitchCamera (Variables|Default|Getowner))
      (CallFunction|AddDialogue "JANE FROG" "We already talked child.")
      (Variables|Default|SetDialogue%20Tree%20Index 5 :!label _label))
    (:7
      (Default|SwitchCamera (Variables|Default|Getowner))
      (CallFunction|AddDialogue "JANE FROG" "We already talked child.")
      (goto _label))
    (:8
      (Default|SwitchCamera (Variables|Default|Getowner))
      (CallFunction|AddDialogue "JANE FROG" "We already talked child.")
      (goto _label))
    (:9
      (Default|SwitchCamera (Variables|Default|Getowner))
      (CallFunction|AddDialogue "JANE FROG" "Don't talk to me ever again.")
      (goto _label))))