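; Base NPC dialogue component that runs branching conversations through a WB_NpcDialogue widget, from opening to delayed close.
; ProgressDialogue advances the tree index when Progress is set, then calls Dialogue, an empty hook presumably overridden per NPC.
; AddDialogue pushes lines to the widget and records chosen options in DialogueProgress, skipping those already recorded.
; ShowOptions spawns focusable option widgets, and UpdateSelectedOption stores the selection and resumes the dialogue.
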(event Custom|Close%20Conversation
  (bind _dialogue_widget (Variables|Default|GetDialogue%20Widget))
  (Variables|Default|SetX%20active false)
  (Default|DecreaseEvent _dialogue_widget)
  (Utilities|FlowControl|Delay 1.0)
  (Widget|RemovefromParent _dialogue_widget)
  (Class|BPINpcInteractable|ClearReferences(Message) (Variables|/Game/UI/NPC_Dialogue/WB_NpcDialogue.WB_NpcDialogue_C|GetPlayer%20Character _dialogue_widget)))

(fn OpenConversation
  (bind _returnvalue (UserInterface|CreateWidget "/Game/UI/NPC_Dialogue/WB_NpcDialogue.WB_NpcDialogue_C" 0 self 0))
  (bind _output_get (Variables|Default|SetDialogue%20Widget _returnvalue))
  (UserInterface|Viewport|AddtoViewport _output_get 0)
  (CallFunction|ProgressDialogue))

(fn ProgressDialogue
  (Default|TriangleSkip (Variables|Default|GetDialogue%20Widget))
  (if (Variables|Default|GetProgress)
    (Math|Integer|IncrementInt (Variables|Default|GetDialogue%20Tree%20Index)
      (:%20%20
        _)))
  (CallFunction|Dialogue))

(fn Dialogue)

(fn AddDialogue
  (params (Npc%20name :type Text) (Dialogue :type Text) (Options :type Array%20of%20Texts) (Option%20chosen :type Integer))
  (bind _output_get (Variables|Default|SetDialogue%20option%20chosen Option%20chosen))
  (if (.ReturnValue (Utilities|Map|Find (Variables|Default|GetDialogue%20Progress) _output_get))
    (return "NewEnumerator0" 0)
    (else
      (Default|UpdateDialogueText (Variables|Default|GetDialogue%20Widget) (Variables|Default|GetDialogue%20Index) Npc%20name Dialogue Options)
      (if (Variables|Default|GetFinished%20Dialogue)
        _
        (elif (Variables|Default|GetProgress)
          _
          (else
            (Utilities|Map|Add (Variables|Default|GetDialogue%20Progress) (Variables|Default|GetDialogue%20option%20chosen) (Variables|Default|GetDialogue%20Tree%20Index)))))
      (return "NewEnumerator1" 0))))

(fn UpdateSelectedOption
  (params (Progress%20Index :type Integer%20%28by%20ref%29) (Option%20Index :type Integer%20%28by%20ref%29))
  (bind _dialogue_widget (Variables|Default|GetDialogue%20Widget))
  (Variables|Default|SetDialogue%20Index Option%20Index)
  (Utilities|Array|Clear (Variables|/Game/UI/NPC_Dialogue/WB_NpcDialogue.WB_NpcDialogue_C|GetOptions%20Entry _dialogue_widget))
  (Widget|Panel|ClearChildren (Variables|/Game/UI/NPC_Dialogue/WB_NpcDialogue.WB_NpcDialogue_C|GetDialogueList _dialogue_widget))
  (Widget|SetVisibility (Variables|/Game/UI/NPC_Dialogue/WB_NpcDialogue.WB_NpcDialogue_C|GetSkipTriangle _dialogue_widget) "Visible")
  (CallFunction|ProgressDialogue))

(fn ClearDialogueProgress
  (Utilities|Map|Clear (Variables|Default|GetDialogue%20Progress)))

(fn RemoveDialogueProgress
  (params (Progress%20Step :type Integer))
  (for _index (range 0 Progress%20Step)
    (Utilities|Map|Remove (Variables|Default|GetDialogue%20Progress) (- (Variables|Default|GetDialogue%20Index) _index))))

(fn SetDialogueTreeIndex
  (params (Dialogue%20Tree%20Index :type Integer))
  (Variables|Default|SetDialogue%20Tree%20Index Dialogue%20Tree%20Index)
  (CallFunction|ClearDialogueProgress))

(fn ShowOptions
  (params (Options :type Array%20of%20Texts))
  (bind _dialogue_widget (Variables|Default|GetDialogue%20Widget))
  (bind _dialogue_widget_2 (Variables|Default|GetDialogue%20Widget))
  (Rendering|Components|TextRender|SetText (Variables|/Game/UI/NPC_Dialogue/WB_NpcDialogue.WB_NpcDialogue_C|GetTxtDialogue _dialogue_widget_2) "")
  (Widget|SetVisibility (Variables|/Game/UI/NPC_Dialogue/WB_NpcDialogue.WB_NpcDialogue_C|GetSkipTriangle _dialogue_widget_2) "Hidden")
  (for (_array_element _array_index) Options
    (bind _returnvalue (UserInterface|CreateWidget "/Game/UI/NPC_Dialogue/WB_DialogueOption.WB_DialogueOption_C" 0 self _array_element _array_index))
    (Widget|Panel|AddChild (Variables|/Game/UI/NPC_Dialogue/WB_NpcDialogue.WB_NpcDialogue_C|GetDialogueList _dialogue_widget) _returnvalue)
    (Utilities|Array|Add (Variables|/Game/UI/NPC_Dialogue/WB_NpcDialogue.WB_NpcDialogue_C|GetOptions%20Entry _dialogue_widget) _returnvalue)
    (Widget|SetKeyboardFocus (Variables|/Game/UI/NPC_Dialogue/WB_DialogueOption.WB_DialogueOption_C|GetBTNoption _returnvalue))))