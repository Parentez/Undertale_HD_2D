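; Dialogue component for the COOL LIZARD NPC, scripting its conversation and remembering how the player first replied.
; The Dialogue function extends its parent and runs a state machine on DialogueTreeIndex: greeting, four reply options, then a branch per reply, one hinting at a lost dog.
; After closing, later talks give a short line matching that choice.
; It also drives camera switches on the owning BP_NPCLizard as the conversation progresses.
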(event EventBeginPlay)

(event EventTick
  (params (DeltaSeconds :type Float%20%28single-precision%29)))

(fn Dialogue
  (|CallParentFunction)
  (switch int (Variables|Default|GetDialogue%20Tree%20Index)
    (:1
      (CallFunction|AddDialogue "COOL LIZARD" "Yo.")
      (bind _asbp_npclizard (Utilities|Casting|CastToBP_NPCLizard (Components|GetOwner)))
      (bind _output_get (Variables|Default|Setowner _asbp_npclizard))
      (Default|SwitchCamera _output_get))
    (:3
      (Variables|Default|SetX%20active false)
      (CallFunction|ShowOptions (Utilities|Array|MakeArray "Hey!" "Yo, dude." "Good morning, sir." "...")))
    (:4
      (Default|SwitchCamera (Variables|Default|Getowner))
      (Variables|Default|SetProgress false)
      (Variables|Default|SetX%20active true)
      (switch int (Variables|Default|GetDialogue%20Index)
        (:0
          (CallFunction|AddDialogue "COOL LIZARD" "Why r u that happy man? Life's tough down here... (smokes cigarette) " 0 1)
          (Variables|Default|SetDialogue%20Tree%20Index 5))
        (:1
          (bind _d_state (CallFunction|AddDialogue "COOL LIZARD" "U look alright. What's a guy like you down here for?" 0 1))
          (switch Utilities|FlowControl|Switch|SwitchonE_NPCDialogueState _d_state
            (:NewEnumerator0
              (CallFunction|AddDialogue "COOL LIZARD" "A dawg? Oh, yeah. Saw one running around ova tha bridge." 0 2)
              (switch Utilities|FlowControl|Switch|SwitchonE_NPCDialogueState "NewEnumerator0"
                (:NewEnumerator0
                  (CallFunction|AddDialogue "COOL LIZARD" "Hope you find the lil guy. " 0 2)
                  (Variables|Default|SetDialogue%20Tree%20Index 5))))))
        (:2
          (CallFunction|AddDialogue "COOL LIZARD" "Man... get outta here..." 0 1)
          (Variables|Default|SetDialogue%20Tree%20Index 5))
        (:3
          (bind _d_state_2 (CallFunction|AddDialogue "COOL LIZARD" "..." 0 1))
          (switch Utilities|FlowControl|Switch|SwitchonE_NPCDialogueState _d_state_2
            (:NewEnumerator0
              (CallFunction|AddDialogue "COOL LIZARD" "..." 0 2)
              (switch Utilities|FlowControl|Switch|SwitchonE_NPCDialogueState "NewEnumerator0"
                (:NewEnumerator0
                  (CallFunction|AddDialogue "COOL LIZARD" "...You're cool." 0 2)
                  (switch Utilities|FlowControl|Switch|SwitchonE_NPCDialogueState "NewEnumerator0"
                    (:NewEnumerator0
                      (CallFunction|AddDialogue "COOL LIZARD" "(you feel almost as cool as COOL LIZARD.)" 0 2)
                      (Variables|Default|SetDialogue%20Tree%20Index 5)))))))))
      (Default|SwitchCamera (Variables|Default|Getowner))
      (Variables|Default|SetFinished%20Dialogue true))
    (:5
      (switch int (Variables|Default|GetDialogue%20Index)
        (:0
          (Variables|Default|SetDialogue%20Tree%20Index 6))
        (:1
          (Variables|Default|SetDialogue%20Tree%20Index 7))
        (:2
          (Variables|Default|SetDialogue%20Tree%20Index 8))
        (:3
          (Variables|Default|SetDialogue%20Tree%20Index 9)))
      (Variables|/Game/Blueprints/NPC/BP_NPC.BP_NPC_C|SetCamera%20switch (Variables|Default|Getowner) 2)
      (CallFunction|CloseConversation))
    (:6
      (Default|SwitchCamera (Variables|Default|Getowner))
      (CallFunction|AddDialogue "COOL LIZARD" "...What?")
      (Variables|Default|SetDialogue%20Tree%20Index 5 :!label _label))
    (:7
      (Default|SwitchCamera (Variables|Default|Getowner))
      (CallFunction|AddDialogue "COOL LIZARD" "Whazzup?")
      (goto _label))
    (:8
      (Default|SwitchCamera (Variables|Default|Getowner))
      (CallFunction|AddDialogue "COOL LIZARD" "(he doesn't even look at you)")
      (goto _label))
    (:9
      (Default|SwitchCamera (Variables|Default|Getowner))
      (CallFunction|AddDialogue "COOL LIZARD" "... (he approves of your coolness)")
      (goto _label))))