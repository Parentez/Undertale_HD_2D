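; BP_NPCTurtle is an interactable turtle NPC that runs dialogue, including a tutorial conversation.
; Interact or the tutorial event opens a conversation through the ACNpcTurtle component, which allows skipping only after a short delay.
; The tutorial event also fetches the player from GM_TopDown, links it to this NPC and disables its movement.
; SkipDialogue advances the component's dialogue once that delay has passed.
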(event Custom|Start%20tutorial%20dialogue
  (bind _asgm_top_down (Utilities|Casting|CastToGM_TopDown (Game|GetGameMode)))
  (bind _output_get (Variables|Default|SetPlayerCharacter (Variables|/Game/Blueprints/GM_TopDown.GM_TopDown_C|GetPlayer%20Character _asgm_top_down)))
  (Variables|Default|SetInteract%20Instigator _output_get)
  (Variables|/Game/Blueprints/MainCharacter/NormalPlayer/BP_PlayerCharacter.BP_PlayerCharacter_C|SetInteractable%20Npc (Variables|/Game/Blueprints/GM_TopDown.GM_TopDown_C|GetPlayer%20Character _asgm_top_down) self)
  (Variables|/Game/Blueprints/MainCharacter/NormalPlayer/BP_PlayerCharacter.BP_PlayerCharacter_C|SetNPC (Variables|Default|GetPlayerCharacter) self)
  (Pawn|Components|CharacterMovement|SetMovementMode (Variables|/Script/Engine.Character|GetCharacterMovement (Variables|Default|GetPlayerCharacter)) "MOVE_None" 0)
  (Variables|Default|SetActivate%20Input true)
  (Default|OpenConversation (Variables|Default|GetAC_NpcTurtle))
  (Utilities|FlowControl|Delay 1.0)
  (Variables|/Game/Blueprints/NPC/AC_NpcDialogue.AC_NpcDialogue_C|SetX%20active (Variables|Default|GetAC_NpcTurtle) true))

(event EventInteract
  (params (Instigator :type Actor%20Object%20Reference))
  (CallFunction|HideEKey)
  (Variables|Default|SetActivate%20Input true)
  (Variables|Default|SetInteract%20Instigator Instigator)
  (Default|OpenConversation (Variables|Default|GetAC_NpcTurtle))
  (Utilities|FlowControl|Delay 1.0)
  (Variables|/Game/Blueprints/NPC/AC_NpcDialogue.AC_NpcDialogue_C|SetX%20active (Variables|Default|GetAC_NpcTurtle) true))

(event EventSkipDialogue
  (if (Variables|/Game/Blueprints/NPC/AC_NpcDialogue.AC_NpcDialogue_C|GetX%20active (Variables|Default|GetAC_NpcTurtle))
    (Development|PrintString "Pressed interact")
    (Default|ProgressDialogue (Variables|Default|GetAC_NpcTurtle))))

(fn ConstructionScript
  (|CallParentFunction))